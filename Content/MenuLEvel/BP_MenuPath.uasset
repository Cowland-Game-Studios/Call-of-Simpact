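; BP_MenuPath is an endlessly growing tiled path that scrolls along negative Y, apparently as menu level background.
; The construction script lays initial meshes 600 units apart up to Index.
; After a short delay, BeginPlay appends one tile at a time, a timeline animating its height, then loops on finish without removing old tiles.
; Tick shifts the root by a fixed per-frame step, so scroll speed depends on frame rate.
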(event EventBeginPlay
  (bind _index (Variables|Default|GetIndex))
  (bind _returnvalue (* _index 600))
  (bind _returnvalue_2 (Math|Conversions|ToFloat(Integer) _returnvalue))
  (Utilities|FlowControl|Delay 0.75)
  (bind _returnvalue_3 (AddComponent|AddStaticMeshComponent false (Math|Transform|MakeTransform (Math|Vector|MakeVector 0.0 _returnvalue_2 -1e+02) "0.000000,180.000000,0.000000" "1.000000,1.000000,1.000000") :!label _label))
  (Math|Integer|IncrementInt _index
    (:%20%20
      (bind _newtile (Timeline|Timeline PlayFromStart)
        (:Update
          (Transformation|SetRelativeLocation _returnvalue_3 (Math|Vector|MakeVector 0.0 _returnvalue_2 _newtile) false false))
        (:Finished
          (goto _label))))))

(event Collision|EventActorBeginOverlap
  (params (OtherActor :type Actor%20Object%20Reference)))

(event EventTick
  (params (DeltaSeconds :type Float%20%28single-precision%29))
  (Transformation|AddRelativeLocation (Variables|Default|GetDefaultSceneRoot) "0.000000,-40.000000,0.000000" false false))

(fn ConstructionScript
  (for _index (range 0 (Variables|Default|GetIndex))
    (AddComponent|AddStaticMeshComponent false (Math|Transform|MakeTransform (Math|Vector|MakeVector 0.0 (Math|Conversions|ToFloat(Integer) (* _index 600)) 0.0) "0.000000,180.000000,0.000000" "1.000000,1.000000,1.000000"))))