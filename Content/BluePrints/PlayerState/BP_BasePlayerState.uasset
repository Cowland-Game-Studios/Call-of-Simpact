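; Base player state that tracks a player's score, deaths and team, with OnRep handlers for replicated changes.
; AddToScore, AddToDeaths and their OnRep counterparts lazily cache the pawn's BP_BaseCharacter and BP_BasePlayerController, then push the new value to the HUD.
; SetTeam and OnRep_Team apply the team color to the pawn's character.
; Setters repeat the OnRep logic, so the caller's machine also updates immediately.
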(fn ConstructionScript)

(fn AddtoScore
  (params (ScoreAmout :type Float%20%28double-precision%29))
  (Variables|Stats|SetPlayerScore (+ (Variables|Stats|GetPlayerScore) ScoreAmout))
  (Utilities|FlowControl|Sequence
    (:then_0
      ;[1 1 1] Check Character
      (Utilities|IsValid (Variables|Player|GetCharacter)
        (:Is%20Valid
          (Variables|Player|SetCharacter (Variables|Player|GetCharacter)))
        (:Is%20Not%20Valid
          (bind _asbp_blaster_character (Utilities|Casting|CastToBP_BaseCharacter (PlayerState|GetPawn)))
          (Variables|Player|SetCharacter _asbp_blaster_character))))
    (:then_1
      ;[1 1 1] Set controller
      (Utilities|IsValid (Variables|Player|GetCharacter)
        (:Is%20Valid
          (Utilities|IsValid (Variables|Player|GetController)
            (:Is%20Valid
              (Variables|Player|SetController (Variables|Player|GetController)))
            (:Is%20Not%20Valid
              (bind _asbp_blaster_player_controller (Utilities|Casting|CastToBP_BasePlayerController (Pawn|GetController (Variables|Player|GetCharacter))))
              (Variables|Player|SetController _asbp_blaster_player_controller))))))
    (:then_2
      ;[1 1 1] Update HUD Score
      (Utilities|IsValid (Variables|Player|GetController)
        (:Is%20Valid
          (Default|SetHUDScore (Variables|Player|GetController) (Variables|Stats|GetPlayerScore)))))))

(fn OnRepPlayerScore
  (Utilities|FlowControl|Sequence
    (:then_0
      ;[1 1 1] Check Character
      (Utilities|IsValid (Variables|Player|GetCharacter)
        (:Is%20Valid
          (Variables|Player|SetCharacter (Variables|Player|GetCharacter)))
        (:Is%20Not%20Valid
          (bind _asbp_blaster_character (Utilities|Casting|CastToBP_BaseCharacter (PlayerState|GetPawn)))
          (Variables|Player|SetCharacter _asbp_blaster_character))))
    (:then_1
      ;[1 1 1] Set controller
      (Utilities|IsValid (Variables|Player|GetCharacter)
        (:Is%20Valid
          (Utilities|IsValid (Variables|Player|GetController)
            (:Is%20Valid
              (Variables|Player|SetController (Variables|Player|GetController)))
            (:Is%20Not%20Valid
              (bind _asbp_blaster_player_controller (Utilities|Casting|CastToBP_BasePlayerController (Pawn|GetController (Variables|Player|GetCharacter))))
              (Variables|Player|SetController _asbp_blaster_player_controller))))))
    (:then_2
      ;[1 1 1] Set Hud Score
      (Utilities|IsValid (Variables|Player|GetController)
        (:Is%20Valid
          (Default|SetHUDScore (Variables|Player|GetController) (Variables|Stats|GetPlayerScore)))))))

(fn OnRepPlayerDeaths
  (Utilities|FlowControl|Sequence
    (:then_0
      ;[1 1 1] Check Character
      (Utilities|IsValid (Variables|Player|GetCharacter)
        (:Is%20Valid
          (Variables|Player|SetCharacter (Variables|Player|GetCharacter)))
        (:Is%20Not%20Valid
          (bind _asbp_blaster_character (Utilities|Casting|CastToBP_BaseCharacter (PlayerState|GetPawn)))
          (Variables|Player|SetCharacter _asbp_blaster_character))))
    (:then_1
      ;[1 1 1] Set controller
      (Utilities|IsValid (Variables|Player|GetCharacter)
        (:Is%20Valid
          (Utilities|IsValid (Variables|Player|GetController)
            (:Is%20Valid
              (Variables|Player|SetController (Variables|Player|GetController)))
            (:Is%20Not%20Valid
              (bind _asbp_blaster_player_controller (Utilities|Casting|CastToBP_BasePlayerController (Pawn|GetController (Variables|Player|GetCharacter))))
              (Variables|Player|SetController _asbp_blaster_player_controller))))))
    (:then_2
      ;[1 1 1] Update HUD Score
      (Utilities|IsValid (Variables|Player|GetController)
        (:Is%20Valid
          (Default|SetHUDDeaths (Variables|Player|GetController) (Variables|Stats|GetPlayerDeaths)))))))

(fn AddtoDeaths
  (params (DeathsAmount :type Integer))
  (Variables|Stats|SetPlayerDeaths (+ (Variables|Stats|GetPlayerDeaths) DeathsAmount))
  (Utilities|FlowControl|Sequence
    (:then_0
      ;[1 1 1] Check Character
      (Utilities|IsValid (Variables|Player|GetCharacter)
        (:Is%20Valid
          (Variables|Player|SetCharacter (Variables|Player|GetCharacter)))
        (:Is%20Not%20Valid
          (bind _asbp_blaster_character (Utilities|Casting|CastToBP_BaseCharacter (PlayerState|GetPawn)))
          (Variables|Player|SetCharacter _asbp_blaster_character))))
    (:then_1
      ;[1 1 1] Set controller
      (Utilities|IsValid (Variables|Player|GetCharacter)
        (:Is%20Valid
          (Utilities|IsValid (Variables|Player|GetController)
            (:Is%20Valid
              (Variables|Player|SetController (Variables|Player|GetController)))
            (:Is%20Not%20Valid
              (bind _asbp_blaster_player_controller (Utilities|Casting|CastToBP_BasePlayerController (Pawn|GetController (Variables|Player|GetCharacter))))
              (Variables|Player|SetController _asbp_blaster_player_controller))))))
    (:then_2
      ;[1 1 1] Update HUD Score
      (Utilities|IsValid (Variables|Player|GetController)
        (:Is%20Valid
          (Default|SetHUDDeaths (Variables|Player|GetController) (Variables|Stats|GetPlayerDeaths)))))))

(fn SetControllerinPlayerState
  (Utilities|FlowControl|Sequence
    (:then_0
      ;[1 1 1] Check Character
      (Utilities|IsValid (Variables|Player|GetCharacter)
        (:Is%20Valid
          (Variables|Player|SetCharacter (Variables|Player|GetCharacter)))
        (:Is%20Not%20Valid
          (bind _asbp_blaster_character (Utilities|Casting|CastToBP_BaseCharacter (PlayerState|GetPawn)))
          (Variables|Player|SetCharacter _asbp_blaster_character))))
    (:then_1
      ;[1 1 1] Set controller
      (Utilities|IsValid (Variables|Player|GetCharacter)
        (:Is%20Valid
          (Utilities|IsValid (Variables|Player|GetController)
            (:Is%20Valid
              (Variables|Player|SetController (Variables|Player|GetController)))
            (:Is%20Not%20Valid
              (bind _asbp_blaster_player_controller (Utilities|Casting|CastToBP_BasePlayerController (Pawn|GetController (Variables|Player|GetCharacter))))
              (Variables|Player|SetController _asbp_blaster_player_controller))))))))

(fn OnRepTeam
  (bind _asbp_blaster_character (Utilities|Casting|CastToBP_BaseCharacter (PlayerState|GetPawn)))
  (bind _output_get (LocalVariables|SetBCharacter _asbp_blaster_character))
  (Utilities|IsValid _output_get
    (:Is%20Valid
      (Default|SetTeamColor _output_get (Variables|Team|GetTeam)))))

(fn SetTeam
  (params (NewParam :type Enum_Teams%20Enum :default "NewEnumerator0"))
  (Variables|Team|SetTeam NewParam)
  (bind _asbp_blaster_character (Utilities|Casting|CastToBP_BaseCharacter (PlayerState|GetPawn)))
  (bind _output_get (LocalVariables|SetBCharacter _asbp_blaster_character))
  (Utilities|IsValid _output_get
    (:Is%20Valid
      (Default|SetTeamColor _output_get (Variables|Team|GetTeam)))))