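; Base HUD that draws the dynamic crosshair and creates the character overlay, announcement and elimination-feed widgets.
; DrawHUD draws up to five HUDPackage textures around screen center, offsetting the outer four by the scaled spread.
; Each elimination message shifts earlier ones up by their canvas slot height.
; A per-message delay then removes it from its parent, though it stays in the ElimMessages array.
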(event Custom|ElimAnnouncementTimer
  (params (MsgToRemove :type WBP%20Elim%20Announcement%20Object%20Reference))
  ;[1 1 1] Delay to delete ElimAnnouncement
  (Utilities|FlowControl|Delay (Variables|ElimAnnouncement|GetElimAnnouncementTime))
  (ElimAnnouncement|ElimAnnouncementTimerFinished MsgToRemove))

(event EventDrawHUD
  (params (SizeX :type Integer) (SizeY :type Integer))
  ;[1 1 1] Draw Hud Crosshair
  (Crosshair|CrossHairManagement))

(fn ConstructionScript)

(fn DrawCrosshair
  (params (Texture :type Texture%202D%20Object%20Reference) (ViewPortCenter :type Vector%202D%20Structure) (Spread :type Vector%202D%20Structure) (CrosshairColorFunction :type Linear%20Color%20Structure))
  (LocalVariables|SetTextureWidth (Math|Conversions|ToFloat(Integer) (Class|Texture2D|BlueprintGetSizeX Texture)))
  (LocalVariables|SetTextureHeight (Math|Conversions|ToFloat(Integer) (Class|Texture2D|BlueprintGetSizeY Texture)))
  (LocalVariables|SetTextureDrawPoint (Math|Vector2D|MakeVector2D (+ (- (.x ViewPortCenter) (/ (LocalVariables|GetTextureWidth) 2.0)) (.x Spread)) (+ (.y Spread) (- (.y ViewPortCenter) (/ (LocalVariables|GetTextureHeight) 2.0)))))
  (Canvas|DrawTexture Texture (.x (LocalVariables|GetTextureDrawPoint)) (.y (LocalVariables|GetTextureDrawPoint)) (LocalVariables|GetTextureWidth) (LocalVariables|GetTextureHeight) 0.0 0.0 1.0 1.0 CrosshairColorFunction))

(fn AddCharacterOverlay
  (bind _characteroverlayclass (Variables|CharacterOverlay|GetCharacterOverlayClass))
  (bind _output_get (LocalVariables|SetPlayerController (Game|Player|GetOwningPlayerController)))
  (Utilities|IsValid _output_get
    (:Is%20Valid
      (if (Utilities|IsValidClass _characteroverlayclass)
        (bind _returnvalue (UserInterface|CreateWidget _characteroverlayclass (LocalVariables|GetPlayerController)))
        (bind _output_get_2 (Variables|CharacterOverlay|SetCharacterOverlay _returnvalue))
        (UserInterface|Viewport|AddtoViewport _output_get_2 0)
        (else
          (Development|PrintString "ERROR AddCharacterOverlay"))))))

(fn CrossHairManagement
  (bind _hudpackage (Variables|Spread|GetHUDPackage))
  (bind (_crosshairscenter _crosshairsright _crosshairsleft _crosshairstop _crosshairsbottom _crosshairspread _crosshairscolor) (Utilities|Struct|BreakHUDCrosshairsPackage _hudpackage))
  (bind _output_get (Variables|ViewPort|SetViewPortSize (Viewport|GetViewportSize)))
  (Variables|ViewPort|SetViewPortCenter (Math|Vector2D|MakeVector2D (/ (.x _output_get) 2.0) (/ (.y _output_get) 2.0)))
  (Variables|Spread|SetSpreadScaled (* (Variables|Spread|GetCrossHairSpreadMax) (.CrossHairSpread (Utilities|Struct|BreakHUDCrosshairsPackage (Variables|Spread|GetHUDPackage)))))
  (Utilities|FlowControl|Sequence
    (:then_0
      (Variables|Spread|SetTempCrosshairColor _crosshairscolor)
      (Utilities|IsValid _crosshairscenter
        (:Is%20Valid
          (bind _output_get_2 (Variables|Spread|SetSpread ""))
          (Crosshair|DrawCrosshair _crosshairscenter (Variables|ViewPort|GetViewPortCenter) _output_get_2 (Variables|Spread|GetTempCrosshairColor)))))
    (:then_1
      (Utilities|IsValid _crosshairsright
        (:Is%20Valid
          (bind _output_get_3 (Variables|Spread|SetSpread (Math|Vector2D|MakeVector2D (Variables|Spread|GetSpreadScaled) 0.0)))
          (Crosshair|DrawCrosshair _crosshairsright (Variables|ViewPort|GetViewPortCenter) _output_get_3 (Variables|Spread|GetTempCrosshairColor)))))
    (:then_2
      (Utilities|IsValid _crosshairsleft
        (:Is%20Valid
          (bind _output_get_4 (Variables|Spread|SetSpread (Math|Vector2D|MakeVector2D (* (Variables|Spread|GetSpreadScaled) -1.0) 0.0)))
          (Crosshair|DrawCrosshair _crosshairsleft (Variables|ViewPort|GetViewPortCenter) _output_get_4 (Variables|Spread|GetTempCrosshairColor)))))
    (:then_3
      (Utilities|IsValid _crosshairstop
        (:Is%20Valid
          (bind _output_get_5 (Variables|Spread|SetSpread (Math|Vector2D|MakeVector2D 0.0 (* (Variables|Spread|GetSpreadScaled) -1.0))))
          (Crosshair|DrawCrosshair _crosshairstop (Variables|ViewPort|GetViewPortCenter) _output_get_5 (Variables|Spread|GetTempCrosshairColor)))))
    (:then_4
      (Utilities|IsValid _crosshairsbottom
        (:Is%20Valid
          (bind _output_get_6 (Variables|Spread|SetSpread (Math|Vector2D|MakeVector2D 0.0 (Variables|Spread|GetSpreadScaled))))
          (Crosshair|DrawCrosshair _crosshairsbottom (Variables|ViewPort|GetViewPortCenter) _output_get_6 (Variables|Spread|GetTempCrosshairColor)))))))

(fn AddAnnouncement
  (bind _announcementclass (Variables|Announcement|GetAnnouncementClass))
  (bind _output_get (LocalVariables|SetPlayerController (Game|Player|GetOwningPlayerController)))
  (Utilities|IsValid _output_get
    (:Is%20Valid
      (if (Utilities|IsValidClass _announcementclass)
        (bind _returnvalue (UserInterface|CreateWidget _announcementclass (LocalVariables|GetPlayerController)))
        (bind _output_get_2 (Variables|Announcement|SetAnnouncement _returnvalue))
        (UserInterface|Viewport|AddtoViewport _output_get_2 0)))))

(fn AddElimAnnouncement
  (params (Attacker :type String) (Victim :type String))
  (bind _elimannouncementclass (Variables|ElimAnnouncement|GetElimAnnouncementClass))
  (Utilities|FlowControl|Sequence
    (:then_0
      (Utilities|IsValid (Variables|Controller|GetOwningPlayer)
        (:Is%20Not%20Valid
          (Variables|Controller|SetOwningPlayer (Game|Player|GetOwningPlayerController)))))
    (:then_1
      (Utilities|IsValid (Variables|Controller|GetOwningPlayer)
        (:Is%20Valid
          (if (Utilities|IsValidClass _elimannouncementclass)
            (bind _returnvalue (UserInterface|CreateWidget _elimannouncementclass (Variables|Controller|GetOwningPlayer)))
            (bind _output_get (Variables|ElimAnnouncement|SetElimAnnouncement _returnvalue))
            (Utilities|IsValid _output_get
              (:Is%20Valid
                (Default|SetElimAnnouncementText _output_get Attacker Victim)
                (UserInterface|Viewport|AddtoViewport _output_get 0)
                (Utilities|FlowControl|Sequence
                  (:then_0
                    (for _array_element (Variables|ElimAnnouncement|GetElimMessages)
                      (Utilities|IsValid _array_element
                        (:Is%20Valid
                          (Utilities|IsValid (Variables|/Game/BluePrints/HUD/WBP_ElimAnnouncement.WBP_ElimAnnouncement_C|GetAnnouncementBox _array_element)
                            (:Is%20Valid
                              (bind _output_get_2 (LocalVariables|SetCanvasSlot (Class|WidgetLayoutLibrary|SlotasCanvasSlot (Variables|/Game/BluePrints/HUD/WBP_ElimAnnouncement.WBP_ElimAnnouncement_C|GetAnnouncementBox _array_element))))
                              (Utilities|IsValid _output_get_2
                                (:Is%20Valid
                                  (bind _output_get_3 (LocalVariables|SetPosition (Class|CanvasPanelSlot|GetPosition _output_get_2)))
                                  (bind _output_get_4 (LocalVariables|SetNewPosition (Math|Vector2D|MakeVector2D (.x _output_get_3) (- (.y _output_get_3) (.y (Class|CanvasPanelSlot|GetSize _output_get_2))))))
                                  (Class|CanvasPanelSlot|SetPosition (LocalVariables|GetCanvasSlot) _output_get_4)))))))))
                  (:then_1
                    (Utilities|Array|Add (Variables|ElimAnnouncement|GetElimMessages) (Variables|ElimAnnouncement|GetElimAnnouncement))
                    (CallFunction|ElimAnnouncementTimer (Variables|ElimAnnouncement|GetElimAnnouncement))))))))))))

(fn ElimAnnouncementTimerFinished
  (params (MsgToRemove :type WBP%20Elim%20Announcement%20Object%20Reference))
  (Utilities|IsValid MsgToRemove
    (:Is%20Valid
      (Widget|RemovefromParent MsgToRemove))))