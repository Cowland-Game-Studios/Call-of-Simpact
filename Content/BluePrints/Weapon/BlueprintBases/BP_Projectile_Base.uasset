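; Base projectile for weapons that spawns a tracer on begin play and impact particles and sound when destroyed.
; On hit, the server applies damage crediting the player or AI controller, while with server-side rewind the locally controlled owner sends hit characters to its lag compensation component for scoring.
; Non-rocket projectiles then destroy themselves.
; Helper functions, not called here, provide a trail system, authority-only radial explosion damage and delayed destruction.
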(event OnComponentHit(CollisionBox)
  (params (HitComponent :type Primitive%20Component%20Object%20Reference) (OtherActor :type Actor%20Object%20Reference) (OtherComp :type Primitive%20Component%20Object%20Reference) (NormalImpulse :type Vector :default "0, 0, 0") (Hit :type Hit%20Result%20Structure%20%28by%20ref%29))
  ;[1 1 1] HIT
  (CallFunction|OnComponentHitFunc OtherActor))

(event EventBeginPlay
  (bind _collisionbox (Variables|Default|GetCollisionBox))
  ;[1 1 1] Begin Play
  (Utilities|IsValid (Variables|Projectile|GetTracer)
    (:Is%20Valid
      (bind _returnvalue (Effects|SpawnEmitterAttached (Variables|Projectile|GetTracer) _collisionbox "None" (Transformation|GetWorldLocation _collisionbox) (Transformation|GetWorldRotation _collisionbox) "1.000000,1.000000,1.000000" "KeepWorldPosition"))
      (Variables|Projectile|SetTracerComponent _returnvalue))))

(event EventDestroyed
  (bind _returnvalue (Transformation|GetActorTransform))
  (bind _impactparticles (Variables|Projectile|GetImpactParticles))
  (bind _impactsound (Variables|Projectile|GetImpactSound))
  ;[1 1 1] on Hit Spawn emitter and sound
  (Utilities|FlowControl|Sequence
    (:then_0
      (Utilities|IsValid _impactparticles
        (:Is%20Valid
          (Effects|SpawnEmitteratLocation _impactparticles (.location _returnvalue) (.rotation _returnvalue) (.scale _returnvalue) false))))
    (:then_1
      (Utilities|IsValid _impactsound
        (:Is%20Valid
          (Audio|PlaySoundatLocation _impactsound (Transformation|GetActorLocation) "0, 0, 0" 1.0 1.0 0.0 0 0 0 0))))))

(fn ConstructionScript)

(fn SpawnTrailSystem
  (bind _trailsystem (Variables|TrailSystem|GetTrailSystem))
  (Utilities|IsValid _trailsystem
    (:Is%20Valid
      (bind _returnvalue (Niagara|SpawnSystemAttached _trailsystem (Variables|Transformation|GetRootComponent) "" (Transformation|GetActorLocation) (Transformation|GetActorRotation) "KeepWorldPosition" false))
      (Variables|TrailSystem|SetTrailSystemComponent _returnvalue))))

(fn DestroyTimerFinished
  (Actor|DestroyActor))

(fn StartDestroyTimer
  (bind _returnvalue (Utilities|Time|SetTimerbyFunctionName 0 "DestroyTimerFinished" (Variables|Timer|GetDestroyTime) true))
  (Variables|Timer|SetDestroyTimer _returnvalue))

(fn ExplodeDamage
  (bind _output_get (Variables|Infos|SetFiringPawn (Game|GetInstigator)))
  (if (and (Utilities|IsValid _output_get) (Ability|HasAuthority))
    (bind _output_get_2 (Variables|Infos|SetFiringController (Pawn|GetController _output_get)))
    (Utilities|IsValid _output_get_2
      (:Is%20Valid
        (Class|GameplayStatics|ApplyRadialDamagewithFalloff (Variables|Damage|GetDamage) 0.0 (Transformation|GetActorLocation) (Variables|Damage|GetDamageInnerRadius) (Variables|Damage|GetDamageOuterRadius) 1.0 "/Script/Engine.DamageType" 0 self (Variables|Infos|GetFiringController) "ECC_Visibility")
        (Timer|StartDestroyTimer)))))

(fn SuperonHit
  (if (not (Variables|Projectile|GetIsRocket))
    (Actor|DestroyActor)))

(fn OnComponentHitFunc
  (params (DamagedUser :type Actor%20Object%20Reference))
  (Utilities|FlowControl|Sequence
    (:then_0
      (Variables|Damage|SetDamagedUser DamagedUser)
      (bind _asbp_base_character (Utilities|Casting|CastToBP_BaseCharacter (Components|GetOwner))
        (:then
          (bind _output_get (Variables|Infos|SetOwnerCharacter _asbp_base_character))
          (Utilities|IsValid _output_get
            (:Is%20Valid
              (if (Class|Pawn|IsControlled _output_get)
                ;[1 1 1] IS a player
                (bind _asbp_base_player_controller (Utilities|Casting|CastToBP_BasePlayerController (Pawn|GetController (Variables|Infos|GetOwnerCharacter)))
                  (:then
                    (bind _output_get_2 (Variables|Infos|SetOwnerController _asbp_base_player_controller))
                    (Utilities|IsValid _output_get_2
                      (:Is%20Valid
                        (Utilities|IsValid (Variables|Damage|GetDamagedUser) :!label _label
                          (:Is%20Valid
                            (Utilities|FlowControl|Sequence
                              (:then_0
                                ;[1 1 1] Not using SSR
                                (if (and (Ability|HasAuthority (Variables|Infos|GetOwnerCharacter)) (not (Variables|ServerSideRewind|GetUseServerSideRewind)))
                                  (if (!= (Variables|Damage|GetDamagedUser) (Variables|Infos|GetOwnerCharacter))
                                    (if (Class|Pawn|IsControlled (Variables|Infos|GetOwnerCharacter))
                                      ;[1 1 1] IS a player
                                      (Game|Damage|ApplyDamage (Variables|Damage|GetDamagedUser) (Variables|Damage|GetDamage) (Variables|Infos|GetOwnerController) self "/Script/Engine.DamageType")
                                      (else
                                        ;;[0.2825 1 0.669] IS a player
                                        (Game|Damage|ApplyDamage (Variables|Damage|GetDamagedUser) (Variables|Damage|GetDamage) (Variables|Default|GetAI_OwnerController) self "/Script/Engine.DamageType")))
                                    (CallFunction|SuperonHit)
                                    (return))))
                              (:then_1
                                (bind _asbp_base_character_2 (Utilities|Casting|CastToBP_BaseCharacter DamagedUser))
                                (LocalVariables|SetHitCharacter _asbp_base_character_2)
                                (if (and (Pawn|IsLocallyControlled (Variables|Infos|GetOwnerCharacter)) (Variables|ServerSideRewind|GetUseServerSideRewind))
                                  (Utilities|IsValid (Variables|/Game/BluePrints/Character/BP_BaseCharacter.BP_BaseCharacter_C|GetLagCompensation_Component (Variables|Infos|GetOwnerCharacter))
                                    (:Is%20Valid
                                      (Utilities|IsValid (LocalVariables|GetHitCharacter)
                                        (:Is%20Valid
                                          (Default|ProjectileServerScoreRequest (Variables|/Game/BluePrints/Character/BP_BaseCharacter.BP_BaseCharacter_C|GetLagCompensation_Component (Variables|Infos|GetOwnerCharacter)) (LocalVariables|GetHitCharacter) (Variables|ServerSideRewind|GetTraceStart) (Variables|ServerSideRewind|GetInitialVelocity) (- (Default|GetServerTime (Variables|Infos|GetOwnerController)) (Variables|/Game/BluePrints/PlayerController/BP_BasePlayerController.BP_BasePlayerController_C|GetSingleTripTime (Variables|Infos|GetOwnerController))))))))))))))))
                  (:CastFailed
                    (Development|PrintString "cast failed")))
                (else
                  ;[0.0769 1 0.371] Is AI
                  (bind _asals_ai_controller (Utilities|Casting|CastToALS_AI_Controller (Pawn|GetController (Variables|Infos|GetOwnerCharacter))))
                  (Variables|Default|SetAI_OwnerController _asals_ai_controller)
                  (goto _label))))))
        (:CastFailed
          (Development|PrintString "owned cast failed"))))
    (:then_1
      (CallFunction|SuperonHit))))