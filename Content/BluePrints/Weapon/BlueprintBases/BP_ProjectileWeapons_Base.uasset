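; Base Blueprint for projectile weapons that spawns a projectile from the muzzle socket toward the hit target on Fire.
; With server-side rewind, the server's local player fires a replicated projectile, while other cases spawn the rewind projectile class, configured by authority and local control.
; The firing client's projectile also records trace start and initial velocity for rewind.
; Without rewind, only the authority spawns the replicated projectile.
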(event EventBeginPlay
  (|CallParentFunction) ; This node is disabled and will not be called.\nDrag off pins to build functionality.
)

(event Collision|EventActorBeginOverlap
  (params (OtherActor :type Actor%20Object%20Reference)))

(event EventTick
  (params (DeltaSeconds :type Float%20%28single-precision%29)))

(fn ConstructionScript
  (|CallParentFunction))

(fn Fire
  (params (HitTarget :type Vector%20%28by%20ref%29 :default "0, 0, 0"))
  (|CallParentFunction HitTarget)
  (bind _aspawn (Utilities|Casting|CastToPawn (Components|GetOwner)))
  (LocalVariables|SetInstigatorPawn _aspawn)
  (Utilities|IsValid (Class|SkeletalMesh|FindSocket (Variables|/Script/Engine.SkinnedMeshComponent|GetSkeletalMesh (Variables|Default|GetWeapon%20Mesh)) (LocalVariables|GetMuzzleSocket))
    (:Is%20Valid
      (bind _output_get (LocalVariables|SetSocketTransform (Transformation|GetSocketTransform (Variables|Default|GetWeapon%20Mesh) (LocalVariables|GetMuzzleSocket) "RTS_World")))
      ;[1 1 1] From Muzzle flash socket to hit location from TraceUnderCrosshairs
      (bind _output_get_2 (LocalVariables|SetToTarget (- HitTarget (.location _output_get))))
      (bind _returnvalue (Class|VectortoRotator|VtoRotator _output_get_2))
      (LocalVariables|SetTargetRotation _returnvalue)
      (if (Variables|Default|GetUseServerSideRewind)
        ;[1 1 1] Using SSR
        ;;[1 0 0] Server
        (if (Ability|HasAuthority (LocalVariables|GetInstigatorPawn))
          ;;[1 0.4102 0.2395] SERVER
          (if (Pawn|IsLocallyControlled (LocalVariables|GetInstigatorPawn))
            ;;;[1 1 1] Server , host - use replicated projectile
            (bind _returnvalue_2 (Game|SpawnActorfromClass (Variables|Default|GetProjectileClass) (Math|Transform|MakeTransform (.location (LocalVariables|GetSocketTransform)) (LocalVariables|GetTargetRotation) (.scale (LocalVariables|GetSocketTransform))) "Undefined" (Components|GetOwner) (LocalVariables|GetInstigatorPawn)))
            (bind _output_get_3 (LocalVariables|SetSpawnedProjectile _returnvalue_2))
            (Variables|/Game/BluePrints/Weapon/BlueprintBases/BP_Projectile_Base.BP_Projectile_Base_C|SetUseServerSideRewind _output_get_3 false)
            (Variables|/Game/BluePrints/Weapon/BlueprintBases/BP_Projectile_Base.BP_Projectile_Base_C|SetDamage _output_get_3 (Variables|Default|GetDamage))
            (else
              ;;;[1 1 1] Server , not localy controlled - spawn nonReplicated projectile , no SSR
              (bind _returnvalue_3 (Game|SpawnActorfromClass (Variables|Default|GetServerSideRewindProjectileClass) (Math|Transform|MakeTransform (.location (LocalVariables|GetSocketTransform)) (LocalVariables|GetTargetRotation) (.scale (LocalVariables|GetSocketTransform))) "Undefined" (Components|GetOwner) (LocalVariables|GetInstigatorPawn)))
              (bind _output_get_4 (LocalVariables|SetSpawnedProjectile _returnvalue_3))
              (Variables|/Game/BluePrints/Weapon/BlueprintBases/BP_Projectile_Base.BP_Projectile_Base_C|SetUseServerSideRewind _output_get_4 true)))
          (else
            ;;[1 0.4102 0.2395] Client Using SSR
            (if (Pawn|IsLocallyControlled (LocalVariables|GetInstigatorPawn))
              ;;;[1 1 1] Client, Locally controlled , spaw non replicated projectile , Use SSR
              (bind _returnvalue_4 (Game|SpawnActorfromClass (Variables|Default|GetServerSideRewindProjectileClass) (Math|Transform|MakeTransform (.location (LocalVariables|GetSocketTransform)) (LocalVariables|GetTargetRotation) (.scale (LocalVariables|GetSocketTransform))) "Undefined" (Components|GetOwner) (LocalVariables|GetInstigatorPawn)))
              (bind _output_get_5 (LocalVariables|SetSpawnedProjectile _returnvalue_4))
              (Variables|/Game/BluePrints/Weapon/BlueprintBases/BP_Projectile_Base.BP_Projectile_Base_C|SetUseServerSideRewind _output_get_5 true)
              (Variables|/Game/BluePrints/Weapon/BlueprintBases/BP_Projectile_Base.BP_Projectile_Base_C|SetTraceStart _output_get_5 (.location (LocalVariables|GetSocketTransform)))
              (Variables|/Game/BluePrints/Weapon/BlueprintBases/BP_Projectile_Base.BP_Projectile_Base_C|SetInitialVelocity _output_get_5 (* (Transformation|GetActorForwardVector _output_get_5) (Variables|/Script/Engine.ProjectileMovementComponent|GetInitialSpeed (Variables|/Game/BluePrints/Weapon/BlueprintBases/BP_Projectile_Base.BP_Projectile_Base_C|GetProjectileMovement _output_get_5))))
              (Variables|/Game/BluePrints/Weapon/BlueprintBases/BP_Projectile_Base.BP_Projectile_Base_C|SetDamage _output_get_5 (Variables|Default|GetDamage))
              (else
                ;;;[1 1 1] Client , not locally controlled - spawn non-replicated projectile , no SSR
                (bind _returnvalue_5 (Game|SpawnActorfromClass (Variables|Default|GetServerSideRewindProjectileClass) (Math|Transform|MakeTransform (.location (LocalVariables|GetSocketTransform)) (LocalVariables|GetTargetRotation) (.scale (LocalVariables|GetSocketTransform))) "Undefined" (Components|GetOwner) (LocalVariables|GetInstigatorPawn)))
                (bind _output_get_6 (LocalVariables|SetSpawnedProjectile _returnvalue_5))
                (Variables|/Game/BluePrints/Weapon/BlueprintBases/BP_Projectile_Base.BP_Projectile_Base_C|SetUseServerSideRewind _output_get_6 false)))))
        (else
          ;[1 1 1] Weapon not using SSR
          ;;[1 1 1] Server , host - use replicated projectile
          (if (Ability|HasAuthority (LocalVariables|GetInstigatorPawn))
            (bind _returnvalue_6 (Game|SpawnActorfromClass (Variables|Default|GetProjectileClass) (Math|Transform|MakeTransform (.location (LocalVariables|GetSocketTransform)) (LocalVariables|GetTargetRotation) (.scale (LocalVariables|GetSocketTransform))) "Undefined" (Components|GetOwner) (LocalVariables|GetInstigatorPawn)))
            (bind _output_get_7 (LocalVariables|SetSpawnedProjectile _returnvalue_6))
            (Variables|/Game/BluePrints/Weapon/BlueprintBases/BP_Projectile_Base.BP_Projectile_Base_C|SetUseServerSideRewind _output_get_7 false)
            (Variables|/Game/BluePrints/Weapon/BlueprintBases/BP_Projectile_Base.BP_Projectile_Base_C|SetDamage _output_get_7 (Variables|Default|GetDamage))))))))