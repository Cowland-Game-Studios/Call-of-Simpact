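; BP_BulletShell_Base is a base Blueprint for a bullet shell, a short-lived physics prop with an impact sound.
; On BeginPlay it enables physics and hit notifications on the shell mesh, then pushes it along the actor's forward vector with an impulse.
; On a hit it plays ShellSound at its location and destroys itself, but only if that sound is valid, so a shell without one remains.
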(event OnComponentHit(BulletShellMesh)
  (params (HitComponent :type Primitive%20Component%20Object%20Reference) (OtherActor :type Actor%20Object%20Reference) (OtherComp :type Primitive%20Component%20Object%20Reference) (NormalImpulse :type Vector :default "0, 0, 0") (Hit :type Hit%20Result%20Structure%20%28by%20ref%29))
  (bind _shellsound (Variables|Default|GetShellSound))
  (Utilities|IsValid _shellsound
    (:Is%20Valid
      (Audio|PlaySoundatLocation _shellsound (Transformation|GetActorLocation) "0, 0, 0" 1.0 1.0 0.0 0 0 0 0)
      (Actor|DestroyActor))))

(event EventBeginPlay
  (bind _bulletshellmesh (Variables|Default|GetBulletShellMesh))
  (Physics|SetSimulatePhysics _bulletshellmesh true)
  (Class|PrimitiveComponent|SetNotifyRigidBodyCollision _bulletshellmesh true)
  (Physics|AddImpulse _bulletshellmesh (Transformation|GetActorForwardVector) "None" false))

(fn ConstructionScript)