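; Base Blueprint for hitscan weapons that deal instant line-trace damage to characters.
; Fire traces from the muzzle socket through and slightly past the target, skipping one weapon type.
; Damage applies on authority, or with server-side rewind, locally controlled clients send timestamped score requests to LagCompensationComponent.
; The trace also drives the beam tracer, impact particles and hit sound, alongside muzzle flash and fire sound.
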(event EventBeginPlay
  (|CallParentFunction) ; This node is disabled and will not be called.\nDrag off pins to build functionality.
)

(event Collision|EventActorBeginOverlap
  (params (OtherActor :type Actor%20Object%20Reference)))

(event EventTick
  (params (DeltaSeconds :type Float%20%28single-precision%29))
  (|CallParentFunction DeltaSeconds) ; This node is disabled and will not be called.\nDrag off pins to build functionality.
)

(fn ConstructionScript
  (|CallParentFunction))

(fn Fire
  (params (HitTarget :type Vector%20%28by%20ref%29 :default "0, 0, 0"))
  (|CallParentFunction HitTarget)
  (if (not (Utilities|Enum|Equal(Enum) (Variables|Default|GetWeaponType) "NewEnumerator6"))
    (WeaponAction|LineTraceDamageEmitter HitTarget)))

(fn LineTraceDamageEmitter
  (params (Hit :type Vector))
  (bind _muzzlesockettransform (Variables|Default|GetMuzzleSocketTransform))
  (bind _muzzleflash (Variables|FiringEffects|GetMuzzleFlash))
  (bind _firesound (Variables|FiringEffects|GetFireSound))
  (bind _hitsound (Variables|FiringEffects|GetHitSound))
  (bind _muzzleflashsocket (Variables|Default|GetMuzzleFlashSocket))
  (bind _weapon_mesh (Variables|Default|GetWeapon%20Mesh))
  (bind _returnvalue (Transformation|GetSocketTransform _weapon_mesh _muzzleflashsocket "RTS_World"))
  ;[1 1 1] Set Owner and Controller
  (bind _aspawn (Utilities|Casting|CastToPawn (Components|GetOwner)))
  (LocalVariables|SetOwnerPawn _aspawn)
  (Utilities|IsValid _aspawn
    (:Is%20Valid
      (LocalVariables|SetInstigatorController (Pawn|GetController _aspawn))
      ;[1 1 1] Muzzle Flash and trace hit
      (Utilities|IsValid (Class|SkeletalMesh|FindSocket (Variables|/Script/Engine.SkinnedMeshComponent|GetSkeletalMesh (Variables|Default|GetWeapon%20Mesh)) _muzzleflashsocket)
        (:Is%20Valid
          (LocalVariables|SetStart (.location _returnvalue))
          (bind _outhit (CallFunction|WeaponTraceHit (.location _returnvalue) Hit))
          (Variables|HitScan|SetOut%20Hit _outhit)
          (LocalVariables|SetEndBeam (LocalVariables|GetEnd))
          (Utilities|FlowControl|Sequence
            (:then_0
              ;[0.3604 0.8287 1] Block Hit Valid
              ;;[1 1 1] Apply Damage
              (Utilities|FlowControl|Sequence
                (:then_0
                  (bind _asbp_base_character (Utilities|Casting|CastToBP_BaseCharacter (.HitActor (Collision|BreakHitResult (Variables|HitScan|GetOut%20Hit)))))
                  (bind _output_get (LocalVariables|SetBaseCharacter _asbp_base_character))
                  (Utilities|IsValid _output_get
                    (:Is%20Valid
                      (Utilities|IsValid (LocalVariables|GetInstigatorController)
                        (:Is%20Valid
                          (Utilities|FlowControl|Sequence
                            (:then_0
                              (if (and (Ability|HasAuthority) (or (not (Variables|Default|GetUseServerSideRewind)) (Pawn|IsLocallyControlled (LocalVariables|GetOwnerPawn))))
                                (Game|Damage|ApplyDamage _output_get (Variables|Default|GetDamage) (LocalVariables|GetInstigatorController) self "/Script/Engine.DamageType")))
                            (:then_1
                              (if (and (not (Ability|HasAuthority)) (Variables|Default|GetUseServerSideRewind))
                                (Utilities|FlowControl|Sequence
                                  (:then_0
                                    (Utilities|IsValid (Variables|Default|GetOwnerCharacter)
                                      (:Is%20Valid
                                        (Variables|Default|SetOwnerCharacter (Variables|Default|GetOwnerCharacter)))
                                      (:Is%20Not%20Valid
                                        (bind _asbp_base_character_2 (Utilities|Casting|CastToBP_BaseCharacter (Components|GetOwner)))
                                        (Variables|Default|SetOwnerCharacter _asbp_base_character_2))))
                                  (:then_1
                                    (Utilities|IsValid (Variables|Default|GetOwnerController)
                                      (:Is%20Valid
                                        (Variables|Default|SetOwnerController (Variables|Default|GetOwnerController)))
                                      (:Is%20Not%20Valid
                                        (bind _asbp_base_player_controller (Utilities|Casting|CastToBP_BasePlayerController (LocalVariables|GetInstigatorController)))
                                        (Variables|Default|SetOwnerController _asbp_base_player_controller))))
                                  (:then_2
                                    (Utilities|IsValid (Variables|Default|GetOwnerController)
                                      (:Is%20Valid
                                        (Utilities|IsValid (Variables|Default|GetOwnerCharacter)
                                          (:Is%20Valid
                                            (Utilities|IsValid (Variables|/Game/BluePrints/Character/BP_BaseCharacter.BP_BaseCharacter_C|GetLagCompensation_Component (Variables|Default|GetOwnerCharacter))
                                              (:Is%20Valid
                                                (if (Pawn|IsLocallyControlled (Variables|Default|GetOwnerCharacter))
                                                  (Default|ServerScoreRequest (Variables|/Game/BluePrints/Character/BP_BaseCharacter.BP_BaseCharacter_C|GetLagCompensation_Component (Variables|Default|GetOwnerCharacter)) (LocalVariables|GetBaseCharacter) (LocalVariables|GetStart) (.ImpactPoint (Collision|BreakHitResult (Variables|HitScan|GetOut%20Hit))) (- (Default|GetServerTime (Variables|Default|GetOwnerController)) (Variables|/Game/BluePrints/PlayerController/BP_BasePlayerController.BP_BasePlayerController_C|GetSingleTripTime (Variables|Default|GetOwnerController))) self))))))))))))))))))
                (:then_1
                  ;;[1 1 1] Spawn Emitter at location
                  (Utilities|IsValid (Variables|FiringEffects|GetImpactParticles)
                    (:Is%20Valid
                      (bind _returnvalue_2 (Class|VectortoRotator|VtoRotator (.ImpactNormal (Collision|BreakHitResult (Variables|HitScan|GetOut%20Hit)))))
                      (Effects|SpawnEmitteratLocation (Variables|FiringEffects|GetImpactParticles) (.ImpactPoint (Collision|BreakHitResult (Variables|HitScan|GetOut%20Hit))) _returnvalue_2 "1.000000,1.000000,1.000000" false "AutoRelease"))))
                (:then_2
                  ;;[1 1 1] Play Sound
                  (Utilities|IsValid _hitsound
                    (:Is%20Valid
                      (Audio|PlaySoundatLocation _hitsound (.ImpactPoint (Collision|BreakHitResult (Variables|HitScan|GetOut%20Hit))) "0, 0, 0" 1.0 1.0 0.0 0 0 0 0))))))
            (:then_1
              ;[1 1 1] Play Muzzle flash Effect
              (Utilities|IsValid _muzzleflash
                (:Is%20Valid
                  (Effects|SpawnEmitteratLocation _muzzleflash (.location _muzzlesockettransform) (.rotation _muzzlesockettransform) (.scale _muzzlesockettransform)))))
            (:then_2
              ;[1 1 1] Fire Sound
              (Utilities|IsValid _firesound
                (:Is%20Valid
                  (Audio|PlaySoundatLocation _firesound (.location (Variables|Default|GetMuzzleSocketTransform)) "0, 0, 0" 1.0 1.0 0.0 0 0 0 0))))))))))

(fn WeaponTraceHit
  (params (TraceStart :type Vector%20%28by%20ref%29) (HitTarget :type Vector%20%28by%20ref%29))
  (bind _beamparticles (Variables|FiringEffects|GetBeamParticles))
  (LocalVariables|SetEnd (+ TraceStart (* (- HitTarget TraceStart) 1.25)))
  (bind _outhit (Collision|LineTraceByChannel TraceStart (LocalVariables|GetEnd) "TraceTypeQuery1" false (Utilities|Array|MakeArray (Components|GetOwner)) "None"))
  (LocalVariables|SetHitresult _outhit)
  (LocalVariables|SetBeamEnd (LocalVariables|GetEnd))
  (Utilities|FlowControl|Sequence
    (:then_0
      (if (.bBlockingHit (Collision|BreakHitResult (LocalVariables|GetHitresult)))
        (LocalVariables|SetBeamEnd (.ImpactPoint (Collision|BreakHitResult (LocalVariables|GetHitresult))))))
    (:then_2
      ;[1 1 1] Beam Tracer
      (Utilities|IsValid _beamparticles
        (:Is%20Valid
          (bind _returnvalue (Effects|SpawnEmitteratLocation _beamparticles TraceStart))
          (Utilities|IsValid _returnvalue
            (:Is%20Valid
              (Effects|Components|ParticleSystem|SetVectorParameter _returnvalue "Target" (LocalVariables|GetBeamEnd)))))))
    (:then_3
      (return (LocalVariables|GetHitresult)))))