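; Base weapon actor for a multiplayer shooter, offering pickup by overlapping characters and handling firing, ammo and HUD updates.
; A replicated weapon state (equipped, secondary, dropped) switches collision, physics, pickup widget and custom-depth outline highlighting.
; Firing plays the mesh animation, ejects a shell and spends a round, with sequence-counted client-side ammo prediction reconciled against server updates.
; A helper computes scattered trace endpoints from the muzzle socket.
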(event OnComponentBeginOverlap(AreaSphere)
  (params (OverlappedComponent :type Primitive%20Component%20Object%20Reference) (OtherActor :type Actor%20Object%20Reference) (OtherComp :type Primitive%20Component%20Object%20Reference) (OtherBodyIndex :type Integer) (bFromSweep :type Boolean) (SweepResult :type Hit%20Result%20Structure%20%28by%20ref%29))
  ;[1 1 1] Overlapping
  (bind _asbp_base_character (Utilities|Casting|CastToBP_BaseCharacter OtherActor))
  (Utilities|IsValid _asbp_base_character
    (:Is%20Valid
      (if (not (and (Utilities|Enum|Equal(Enum) (Variables|WeaponProperties|GetWeaponType) "NewEnumerator9") (Utilities|Enum|Equal(Enum) (Default|GetTeam _asbp_base_character) (Variables|Flag|GetFlagTeam))))
        (Default|SetOverlappingWeapon _asbp_base_character self true)
        (Variables|/Game/BluePrints/Character/BP_BaseCharacter.BP_BaseCharacter_C|SetLast_Weapon _asbp_base_character self)))))

(event OnComponentEndOverlap(AreaSphere)
  (params (OverlappedComponent :type Primitive%20Component%20Object%20Reference) (OtherActor :type Actor%20Object%20Reference) (OtherComp :type Primitive%20Component%20Object%20Reference) (OtherBodyIndex :type Integer))
  ;[1 1 1] End Overlapping
  (bind _asbp_base_character (Utilities|Casting|CastToBP_BaseCharacter OtherActor))
  (Utilities|IsValid _asbp_base_character
    (:Is%20Valid
      (if (not (and (Utilities|Enum|Equal(Enum) (Variables|WeaponProperties|GetWeaponType) "NewEnumerator9") (Utilities|Enum|Equal(Enum) (Default|GetTeam _asbp_base_character) (Variables|Flag|GetFlagTeam))))
        (Variables|/Game/BluePrints/Character/BP_BaseCharacter.BP_BaseCharacter_C|SetLast_Weapon _asbp_base_character 0)
        (Default|SetOverlappingWeapon _asbp_base_character 0 false)))))

(event Custom|ClientUpdateAmmo
  (params (ServerAmmo :type Integer))
  ;[1 1 1] Client Side predicting ammo
  (if (not (Ability|HasAuthority))
    (Variables|WeaponProperties|SetAmmo ServerAmmo)
    (bind _result (Math|Integer|DecrementInt (Variables|PredictingAmmo|GetSequence))
      (:%20%20
        (Variables|WeaponProperties|SetAmmo (- (Variables|WeaponProperties|GetAmmo) _result))
        (Ammo|SetHUDAmmo)))))

(event Custom|ClientAddAmmo
  (params (AmmoToAdd :type Integer))
  ;[1 1 1] Client Side predicting ammo
  (if (not (Ability|HasAuthority))
    (Variables|WeaponProperties|SetAmmo (Math|Integer|Clamp(Integer) (+ (Variables|WeaponProperties|GetAmmo) AmmoToAdd) 0 (Variables|WeaponProperties|GetMagCapacity)))
    (Ammo|SetHUDAmmo)))

(event EventBeginPlay
  ;[1 1 1] Begin Play
  (if (Utilities|Enum|Equal(Enum) (Variables|WeaponProperties|GetWeaponType) "NewEnumerator7")
    (Transformation|SetRelativeLocation (Variables|Default|GetScopeCamera) (Math|Vector|MakeVector 0.0 (Variables|Scope|GetMaxScopeRange) 0.0) true false)))

(fn ConstructionScript
  (bind _area_sphere (Variables|WeaponComposition|GetArea%20Sphere))
  (bind _pickup_widget (Variables|WeaponComposition|GetPickUp%20Widget))
  (Utilities|FlowControl|Sequence
    (:then_0
      (if (Ability|HasAuthority)
        (Collision|SetCollisionEnabled _area_sphere "QueryAndPhysics")
        (Collision|SetCollisionResponsetoChannel _area_sphere "ECC_Pawn" "ECR_Overlap")))
    (:then_1
      (Utilities|IsValid _pickup_widget
        (:Is%20Valid
          (Rendering|SetVisibility _pickup_widget false false))))
    (:then_2
      ;[1 1 1] Weapon HighLight
      (Rendering|SetCustomDepthStencilValue (Variables|WeaponComposition|GetWeapon%20Mesh) (Variables|/Game/BluePrints/Components/BP_Component_GlobalVariables.BP_Component_GlobalVariables_C|GetCUSTOM_DEPTH_BLUE (Variables|Default|GetBP_Component_GlobalVariables)))
      (Rendering|SetRenderCustomDepth (Variables|WeaponComposition|GetWeapon%20Mesh) true))))

(fn SetWeaponState
  (params (State :type ENUM_WeaponState%20Enum :default "NewEnumerator0"))
  (Variables|WeaponProperties|SetWeaponStateN State)
  (WeaponState|OnWeaponStateSet))

(fn ShowPickUpWidget
  (params (ShowWidgetState :type Boolean))
  (bind _pickup_widget (Variables|WeaponComposition|GetPickUp%20Widget))
  (Utilities|IsValid _pickup_widget
    (:Is%20Valid
      (Rendering|SetVisibility _pickup_widget ShowWidgetState false))))

(fn Fire
  (params (HitTarget :type Vector%20%28by%20ref%29))
  (bind _buleltshell (Variables|BulletShell|GetBuleltShell))
  (bind _weaponfireanimation (Variables|WeaponComposition|GetWeaponFireAnimation))
  (Utilities|FlowControl|Sequence
    (:then_0
      (Utilities|IsValid _weaponfireanimation
        (:Is%20Valid
          (Components|Animation|PlayAnimation (Variables|WeaponComposition|GetWeapon%20Mesh) _weaponfireanimation false)
          (Utilities|IsValid (Class|SkeletalMesh|FindSocket (Variables|/Script/Engine.SkinnedMeshComponent|GetSkeletalMesh (Variables|WeaponComposition|GetWeapon%20Mesh)) (Variables|BulletShell|GetAmmoEject))
            (:Is%20Valid
              (LocalVariables|SetAmmoEjectTransform (Transformation|GetSocketTransform (Variables|WeaponComposition|GetWeapon%20Mesh) (Variables|BulletShell|GetAmmoEject) "RTS_World"))
              (if (Utilities|IsValidClass _buleltshell)
                (Game|SpawnActorfromClass _buleltshell (LocalVariables|GetAmmoEjectTransform) "AdjustIfPossibleButAlwaysSpawn" self 0)))))))
    (:then_1
      (Ammo|SpendRound))))

(fn NetRoleShow
  (bind _area_sphere (Variables|WeaponComposition|GetArea%20Sphere))
  (bind _pickup_widget (Variables|WeaponComposition|GetPickUp%20Widget))
  (if (Ability|HasAuthority)
    (Collision|SetCollisionEnabled _area_sphere "QueryAndPhysics")
    (Collision|SetCollisionResponsetoChannel _area_sphere "ECC_Pawn" "ECR_Overlap")
    (Utilities|IsValid _pickup_widget
      (:Is%20Valid
        (Rendering|SetVisibility _pickup_widget false false))
      (:Is%20Not%20Valid
        (Development|PrintString "Not valid")))))

(fn Dropped
  (Variables|WeaponProperties|SetWeaponStateN "NewEnumerator2")
  (Transformation|DetachFromComponent (Variables|WeaponComposition|GetWeapon%20Mesh) "KeepWorld" "KeepWorld" "KeepWorld" false)
  (Actor|SetOwner 0)
  (Collision|SetCollisionEnabled (Variables|WeaponComposition|GetArea%20Sphere) "QueryAndPhysics")
  (Variables|Owner|SetOwnerRep 0)
  (Variables|Owner|SetOwnerCharacter 0)
  (Variables|Owner|SetOwnerController 0))

(fn OnRepWeaponStateN
  (WeaponState|OnWeaponStateSet))

(fn AddAmmo
  (params (AmmoToAdd :type Integer))
  (Variables|WeaponProperties|SetAmmo (Math|Integer|Clamp(Integer) (+ (Variables|WeaponProperties|GetAmmo) AmmoToAdd) 0 (Variables|WeaponProperties|GetMagCapacity)))
  (Ammo|SetHUDAmmo)
  (CallFunction|ClientAddAmmo AmmoToAdd))

(fn SpendRound
  (Utilities|FlowControl|Sequence
    (:then_0
      ;[1 1 1] --- Ammo
      (Variables|WeaponProperties|SetAmmo (Math|Integer|Clamp(Integer) (- (Variables|WeaponProperties|GetAmmo) 1) 0 (Variables|WeaponProperties|GetMagCapacity))))
    (:then_1
      (Ammo|SetHUDAmmo))
    (:then_2
      (if (Ability|HasAuthority)
        (CallFunction|ClientUpdateAmmo (Variables|WeaponProperties|GetAmmo))
        (else
          (Math|Integer|IncrementInt (Variables|PredictingAmmo|GetSequence)))))))

(fn SetHUDAmmo
  (Utilities|FlowControl|Sequence
    (:then_0
      ;[1 1 1] Set Owner Character
      (Utilities|IsValid (Variables|Owner|GetOwnerCharacter)
        (:Is%20Valid
          (Variables|Owner|SetOwnerCharacter (Variables|Owner|GetOwnerCharacter)))
        (:Is%20Not%20Valid
          (bind _asbp_base_character (Utilities|Casting|CastToBP_BaseCharacter (Components|GetOwner)))
          (Variables|Owner|SetOwnerCharacter _asbp_base_character))))
    (:then_1
      ;[1 1 1] Set Controller
      (Utilities|IsValid (Variables|Owner|GetOwnerCharacter)
        (:Is%20Valid
          (Utilities|IsValid (Variables|Owner|GetOwnerController)
            (:Is%20Valid
              (Variables|Owner|SetOwnerController (Variables|Owner|GetOwnerController)))
            (:Is%20Not%20Valid
              (bind _asbp_base_player_controller (Utilities|Casting|CastToBP_BasePlayerController (Pawn|GetController (Variables|Owner|GetOwnerCharacter))))
              (Variables|Owner|SetOwnerController _asbp_base_player_controller))))))
    (:then_2
      ;[1 1 1] Set Hud weapon ammo
      (Utilities|IsValid (Variables|Owner|GetOwnerController)
        (:Is%20Valid
          (Default|SetHUDWeaponAmmo (Variables|Owner|GetOwnerController) (Variables|WeaponProperties|GetAmmo)))))))

(fn OnRepOwnerRep
  (Utilities|FlowControl|Sequence
    (:then_0
      ;[1 1 1] Reset character and controller ( owner)
      (if (or (== (Components|GetOwner) 0) (== (Variables|Owner|GetOwnerRep) 0))
        (Variables|Owner|SetOwnerCharacter 0)
        (Variables|Owner|SetOwnerController 0)
        (else
          (Utilities|FlowControl|Sequence
            (:then_0
              (Utilities|IsValid (Variables|Owner|GetOwnerCharacter)
                (:Is%20Valid
                  (Variables|Owner|SetOwnerCharacter (Variables|Owner|GetOwnerCharacter)))
                (:Is%20Not%20Valid
                  (bind _asbp_base_character (Utilities|Casting|CastToBP_BaseCharacter (Components|GetOwner)))
                  (Variables|Owner|SetOwnerCharacter _asbp_base_character))))
            (:then_1
              (Utilities|IsValid (Variables|Owner|GetOwnerCharacter)
                (:Is%20Valid
                  (Utilities|IsValid (Variables|/Game/BluePrints/Components/BP_Component_Combat.BP_Component_Combat_C|GetEquippedWeapon (Variables|/Game/AdvancedLocomotionV4/Blueprints/CharacterLogic/ALS_AnimMan_CharacterBP.ALS_AnimMan_CharacterBP_C|GetCombat (Variables|Owner|GetOwnerCharacter)))
                    (:Is%20Valid
                      (if (== (Variables|/Game/BluePrints/Components/BP_Component_Combat.BP_Component_Combat_C|GetEquippedWeapon (Variables|/Game/AdvancedLocomotionV4/Blueprints/CharacterLogic/ALS_AnimMan_CharacterBP.ALS_AnimMan_CharacterBP_C|GetCombat (Variables|Owner|GetOwnerCharacter))) self)
                        (Ammo|SetHUDAmmo)))))))))))))

(fn IsEmpty
  (return (<= (Variables|WeaponProperties|GetAmmo) 0)))

(fn PlayEmptySound
  (params (combatState :type ENUM_CombatState%20Enum :default "NewEnumerator0"))
  (bind _emptymagazinesound (Variables|Sounds|GetEmptyMagazineSound))
  (bind _isempty_ (Ammo|IsEmpty))
  (if (and _isempty_ (Utilities|Enum|NotEqual(Enum) combatState "NewEnumerator2"))
    (Utilities|IsValid _emptymagazinesound
      (:Is%20Valid
        (Audio|PlaySoundatLocation _emptymagazinesound (Transformation|GetSocketLocation (Variables|WeaponComposition|GetWeapon%20Mesh) "AmmoEject") "0, 0, 0" 1.0 1.0 0.0 0 0 0 0)))))

(fn ReloadSound
  (params (Sound :type Sound%20Base%20Object%20Reference))
  (Utilities|IsValid Sound
    (:Is%20Valid
      (Audio|PlaySoundatLocation Sound (Transformation|GetActorLocation (Variables|Owner|GetOwnerCharacter)) "0, 0, 0" 1.0 1.0 0.0 0 0 0 0))))

(fn AddCustomDepth
  (params (Enable :type Boolean))
  (bind _weapon_mesh (Variables|WeaponComposition|GetWeapon%20Mesh))
  (Utilities|IsValid _weapon_mesh
    (:Is%20Valid
      (Rendering|SetRenderCustomDepth _weapon_mesh Enable))))

(fn IsFull
  (return (== (Variables|WeaponProperties|GetMagCapacity) (Variables|WeaponProperties|GetAmmo))))

(fn OnWeaponStateSet
  (switch Utilities|FlowControl|Switch|SwitchonENUM_WeaponState (Variables|WeaponProperties|GetWeaponStateN)
    (:NewEnumerator1
      (WeaponState|OnEquipped))
    (:NewEnumerator5
      (WeaponState|OnEquippedSecondary))
    (:NewEnumerator2
      (WeaponState|OnDropped))))

(fn OnEquipped
  (bind _weapon_mesh (Variables|WeaponComposition|GetWeapon%20Mesh))
  (Utilities|FlowControl|Sequence
    (:then_0
      ;[1 1 1] Equipped Weapon
      (Widget|ShowPickUpWidget false)
      (Collision|SetCollisionEnabled (Variables|WeaponComposition|GetArea%20Sphere) "NoCollision")
      (Physics|SetSimulatePhysics _weapon_mesh false)
      (Physics|SetEnableGravity _weapon_mesh false)
      (Collision|SetCollisionEnabled _weapon_mesh "NoCollision")
      (if (Utilities|Enum|Equal(Enum) (Variables|WeaponProperties|GetWeaponType) "NewEnumerator5")
        (Collision|SetCollisionEnabled _weapon_mesh "QueryAndPhysics")
        (Physics|SetEnableGravity _weapon_mesh true)
        (Collision|SetCollisionResponsetoAllChannels _weapon_mesh "ECR_Ignore")))
    (:then_1
      (WeaponHalo|AddCustomDepth false))))

(fn OnEquippedSecondary
  (bind _weapon_mesh (Variables|WeaponComposition|GetWeapon%20Mesh))
  (bind _weapon_mesh_2 (Variables|WeaponComposition|GetWeapon%20Mesh))
  (Utilities|FlowControl|Sequence
    (:then_0
      ;[1 1 1] Equipped Weapon
      (Widget|ShowPickUpWidget false)
      (Collision|SetCollisionEnabled (Variables|WeaponComposition|GetArea%20Sphere) "NoCollision")
      (Physics|SetSimulatePhysics _weapon_mesh false)
      (Physics|SetEnableGravity _weapon_mesh false)
      (Collision|SetCollisionEnabled _weapon_mesh "NoCollision")
      (if (Utilities|Enum|Equal(Enum) (Variables|WeaponProperties|GetWeaponType) "NewEnumerator5")
        (Collision|SetCollisionEnabled _weapon_mesh "QueryAndPhysics")
        (Physics|SetEnableGravity _weapon_mesh true)
        (Collision|SetCollisionResponsetoAllChannels _weapon_mesh "ECR_Ignore")))
    (:then_2
      ;[1 1 1] Weapon HighLight
      (Utilities|IsValid _weapon_mesh_2
        (:Is%20Valid
          (Rendering|SetCustomDepthStencilValue _weapon_mesh_2 (Variables|/Game/BluePrints/Components/BP_Component_GlobalVariables.BP_Component_GlobalVariables_C|GetCUSTOM_DEPTH_TAN (Variables|Default|GetBP_Component_GlobalVariables)))
          (Rendering|SetRenderCustomDepth _weapon_mesh_2 true))))))

(fn OnDropped
  (bind _weapon_mesh (Variables|WeaponComposition|GetWeapon%20Mesh))
  (bind _weapon_mesh_2 (Variables|WeaponComposition|GetWeapon%20Mesh))
  ;[1 1 1] Dropped Weapon
  (Utilities|FlowControl|Sequence
    (:then_0
      (if (Ability|HasAuthority)
        (Collision|SetCollisionEnabled (Variables|WeaponComposition|GetArea%20Sphere) "QueryOnly")))
    (:then_1
      (Physics|SetSimulatePhysics _weapon_mesh_2 true)
      (Physics|SetEnableGravity _weapon_mesh_2 true)
      (Collision|SetCollisionEnabled _weapon_mesh_2 "QueryAndPhysics")
      (Collision|SetCollisionResponsetoAllChannels _weapon_mesh_2 "ECR_Block")
      (Collision|SetCollisionResponsetoChannel _weapon_mesh_2 "ECC_Pawn" "ECR_Ignore")
      (Collision|SetCollisionResponsetoChannel _weapon_mesh_2 "ECC_Camera" "ECR_Ignore")
      ;[1 1 1] Weapon HighLight
      (Utilities|IsValid _weapon_mesh
        (:Is%20Valid
          (Rendering|SetCustomDepthStencilValue _weapon_mesh (Variables|/Game/BluePrints/Components/BP_Component_GlobalVariables.BP_Component_GlobalVariables_C|GetCUSTOM_DEPTH_BLUE (Variables|Default|GetBP_Component_GlobalVariables)))
          (Rendering|SetRenderCustomDepth _weapon_mesh true))))))

(fn TraceEndwithScatter
  (params (HitTarget :type Vector%20%28by%20ref%29))
  (bind _muzzleflashsocket (Variables|Muzzle|GetMuzzleFlashSocket))
  (bind _bp_component_globalvariables (Variables|Default|GetBP_Component_GlobalVariables))
  ;[1 1 1] Get socket
  (Utilities|IsValid (Class|SkeletalMesh|FindSocket (Variables|/Script/Engine.SkinnedMeshComponent|GetSkeletalMesh (Variables|WeaponComposition|GetWeapon%20Mesh)) _muzzleflashsocket)
    (:Is%20Valid
      (bind _output_get (Variables|Muzzle|SetMuzzleSocketTransform (Transformation|GetSocketTransform (Variables|WeaponComposition|GetWeapon%20Mesh) _muzzleflashsocket "RTS_World")))
      (LocalVariables|SetTraceStart (.location _output_get))
      (bind _output_get_2 (LocalVariables|SetToTargetNormalized (Math|Vector|Normalize (- HitTarget (LocalVariables|GetTraceStart)))))
      (LocalVariables|SetSphereCenter (+ (* _output_get_2 (Variables|WeaponSpread|GetDistanceToSphere)) (LocalVariables|GetTraceStart)))
      (bind _output_get_3 (LocalVariables|SetRandVec (* (Math|Random|RandomUnitVector) (Math|Random|RandomFloatinRange 0.0 (Variables|WeaponSpread|GetSphereRadius)))))
      (bind _output_get_4 (LocalVariables|SetEndLoc (+ _output_get_3 (LocalVariables|GetSphereCenter))))
      (LocalVariables|SetToEndLoc (- _output_get_4 (LocalVariables|GetTraceStart)))
      (Utilities|IsValid _bp_component_globalvariables
        (:Is%20Valid
          (bind _returnvalue (Class|VectortoRotator|VecSize (LocalVariables|GetToEndLoc)))
          (return (+ (/ (* (LocalVariables|GetToEndLoc) (Variables|/Game/BluePrints/Components/BP_Component_GlobalVariables.BP_Component_GlobalVariables_C|GetTRACE_LENGTH _bp_component_globalvariables)) _returnvalue) (LocalVariables|GetTraceStart))))
        (:Is%20Not%20Valid
          (Development|PrintString "Tracer LENGTH NOT VALID"))))
    (:Is%20Not%20Valid
      (return "0, 0, 0"))))