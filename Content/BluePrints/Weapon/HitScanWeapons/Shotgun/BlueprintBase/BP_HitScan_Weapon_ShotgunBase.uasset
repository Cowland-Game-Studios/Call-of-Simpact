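; Base hitscan shotgun weapon that fires multiple scattered pellets per shot with networked hit registration.
; ShotgunTraceEndWithScater builds pellet targets from random points in a sphere along the aim, extended to trace length.
; FireShotgun traces each target, plays impact effects and counts hits per character, so authority applies damage once per victim, scaled by hits.
; With server-side rewind, locally controlled clients send hits and estimated server time to LagCompensationComponent for scoring.
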(event EventBeginPlay
  (|CallParentFunction) ; This node is disabled and will not be called.\nDrag off pins to build functionality.
)

(event Collision|EventActorBeginOverlap
  (params (OtherActor :type Actor%20Object%20Reference))
  (|CallParentFunction OtherActor) ; This node is disabled and will not be called.\nDrag off pins to build functionality.
)

(event EventTick
  (params (DeltaSeconds :type Float%20%28single-precision%29))
  (|CallParentFunction DeltaSeconds) ; This node is disabled and will not be called.\nDrag off pins to build functionality.
)

(fn ConstructionScript
  (|CallParentFunction))

(fn ShotgunTraceEndwithScater
  (params (HitTarget :type Vector%20%28by%20ref%29) (HitTargets :type Array%20of%20Vector%20Net%20Quantize%20Structures))
  (bind _muzzleflashsocket (Variables|Default|GetMuzzleFlashSocket))
  (bind _bp_component_globalvariables (Variables|Default|GetBP_Component_GlobalVariables))
  (Utilities|FlowControl|Sequence
    (:then_0
      ;[1 1 1] Get socket
      (Utilities|IsValid (Class|SkeletalMesh|FindSocket (Variables|/Script/Engine.SkinnedMeshComponent|GetSkeletalMesh (Variables|Default|GetWeapon%20Mesh)) _muzzleflashsocket)
        (:Is%20Valid
          (bind _output_get (Variables|Default|SetMuzzleSocketTransform (Transformation|GetSocketTransform (Variables|Default|GetWeapon%20Mesh) _muzzleflashsocket "RTS_World")))
          (LocalVariables|SetTraceStart (.location _output_get))
          (bind _output_get_2 (LocalVariables|SetToTargetNormalized (Math|Vector|Normalize (- HitTarget (LocalVariables|GetTraceStart)))))
          (LocalVariables|SetSphereCenter (+ (* _output_get_2 (Variables|Default|GetDistanceToSphere)) (LocalVariables|GetTraceStart))))
        (:Is%20Not%20Valid
          (return "0, 0, 0"))))
    (:then_1
      (for _index (range 0 (- (Variables|WeaponSpread|GetNumberOfPellets) 1))
        (CallFunction|TraceEndwithScatter HitTarget)
        (bind _output_get_3 (LocalVariables|SetRandVec (* (Math|Random|RandomUnitVector) (Math|Random|RandomFloatinRange 0.0 (Variables|Default|GetSphereRadius)))))
        (bind _output_get_4 (LocalVariables|SetEndLoc (+ _output_get_3 (LocalVariables|GetSphereCenter))))
        (LocalVariables|SetToEndLoc (- _output_get_4 (LocalVariables|GetTraceStart)))
        (Utilities|IsValid _bp_component_globalvariables
          (:Is%20Valid
            (bind _returnvalue (Class|VectortoRotator|VecSize (LocalVariables|GetToEndLoc)))
            (bind _output_get_5 (LocalVariables|SetToEndLoc (+ (/ (* (LocalVariables|GetToEndLoc) (Variables|/Game/BluePrints/Components/BP_Component_GlobalVariables.BP_Component_GlobalVariables_C|GetTRACE_LENGTH _bp_component_globalvariables)) _returnvalue) (LocalVariables|GetTraceStart))))
            (Utilities|Array|Add HitTargets (Math|Vector|MakeVectorNetQuantize (.x _output_get_5) (.y _output_get_5) (.z _output_get_5)))))))))

(fn FireShotgun
  (params (HitTargetsInput :type Array%20of%20Vector%20Net%20Quantize%20Structures))
  (bind _hitmap (LocalVariables|GetHitMap))
  (bind _hitmap_2 (LocalVariables|GetHitMap))
  (bind _hitsound (Variables|Default|GetHitSound))
  (bind _muzzleflashsocket_0 (Variables|Default|GetMuzzleFlashSocket_0))
  ;[1 1 1] Set Instigator controller
  (|CallParentFunction (Math|Vector|MakeVectorNetQuantize 0.0 0.0 0.0))
  (bind _aspawn (Utilities|Casting|CastToPawn (Components|GetOwner)))
  (LocalVariables|SetOwnerPawn _aspawn)
  (Utilities|IsValid _aspawn
    (:Is%20Valid
      (LocalVariables|SetInstigatorController (Pawn|GetController _aspawn))
      ;[1 1 1] Get socket
      (Utilities|IsValid (Class|SkeletalMesh|FindSocket (Variables|/Script/Engine.SkinnedMeshComponent|GetSkeletalMesh (Variables|Default|GetWeapon%20Mesh)) _muzzleflashsocket_0)
        (:Is%20Valid
          (bind _output_get (LocalVariables|SetSocketTransform (Transformation|GetSocketTransform (Variables|Default|GetWeapon%20Mesh) _muzzleflashsocket_0 "RTS_World")))
          (LocalVariables|SetStart (.location _output_get))
          (for _array_element HitTargetsInput
            (bind _outhit (CallFunction|WeaponTraceHit (LocalVariables|GetStart) _array_element))
            (bind _output_get_2 (LocalVariables|SetHitResult _outhit))
            ;[1 1 1] save hits actors
            (Utilities|FlowControl|Sequence
              (:then_0
                (bind _asbp_base_character (Utilities|Casting|CastToBP_BaseCharacter (.HitActor (Collision|BreakHitResult _output_get_2))))
                (bind _output_get_3 (LocalVariables|SetBaseCharacter _asbp_base_character))
                (Utilities|IsValid _output_get_3
                  (:Is%20Valid
                    (if (Utilities|Map|Contains _hitmap (LocalVariables|GetBaseCharacter))
                      (bind _result (Math|Integer|IncrementInt (.Value (Utilities|Map|Find _hitmap (LocalVariables|GetBaseCharacter))))
                        (:%20%20
                          (Utilities|Map|Add _hitmap (LocalVariables|GetBaseCharacter) _result)))
                      (else
                        (Utilities|Map|Add _hitmap (LocalVariables|GetBaseCharacter) 1))))))
              (:then_1
                ;[1 1 1] Spawn Emitter at location
                (Utilities|IsValid (Variables|Default|GetImpactParticles)
                  (:Is%20Valid
                    (bind _returnvalue (Class|VectortoRotator|VtoRotator (.ImpactNormal (Collision|BreakHitResult (LocalVariables|GetHitResult)))))
                    (Effects|SpawnEmitteratLocation (Variables|Default|GetImpactParticles) (.ImpactPoint (Collision|BreakHitResult (LocalVariables|GetHitResult))) _returnvalue "1.000000,1.000000,1.000000" false "AutoRelease"))))
              (:then_2
                ;[1 1 1] Play Sound
                (Utilities|IsValid _hitsound
                  (:Is%20Valid
                    (Audio|PlaySoundatLocation _hitsound (.ImpactPoint (Collision|BreakHitResult (LocalVariables|GetHitResult))) "0, 0, 0" 0.5 (Math|Random|RandomFloatinRange -5.0 5.0) 0.0 0 0 0 0))))))
          ;[1 1 1] Apply dammage
          (bind _keys (Utilities|Map|Keys _hitmap_2))
          (for _array_element_2 _keys
            (if (and (.ReturnValue (Utilities|Map|Find _hitmap_2 _array_element_2)) (Utilities|IsValid (LocalVariables|GetInstigatorController)))
              (Utilities|FlowControl|Sequence
                (:then_0
                  (if (and (Ability|HasAuthority) (or (not (Variables|Default|GetUseServerSideRewind)) (Pawn|IsLocallyControlled (LocalVariables|GetOwnerPawn))))
                    (Game|Damage|ApplyDamage _array_element_2 (* (Variables|Default|GetDamage) (.Value (Utilities|Map|Find _hitmap_2 _array_element_2))) (LocalVariables|GetInstigatorController) self "/Script/Engine.DamageType")))
                (:then_1
                  ;;[1 1 1] Add characters
                  (Utilities|Array|Add (LocalVariables|GetHitCharacters) _array_element_2)))))
          (if (and (not (Ability|HasAuthority)) (Variables|Default|GetUseServerSideRewind))
            (Utilities|FlowControl|Sequence
              (:then_0
                (Utilities|IsValid (Variables|Default|GetOwnerCharacter)
                  (:Is%20Valid
                    (Variables|Default|SetOwnerCharacter (Variables|Default|GetOwnerCharacter)))
                  (:Is%20Not%20Valid
                    (bind _asbp_base_character_2 (Utilities|Casting|CastToBP_BaseCharacter (Components|GetOwner)))
                    (Variables|Default|SetOwnerCharacter _asbp_base_character_2))))
              (:then_1
                (Utilities|IsValid (Variables|Default|GetOwnerController)
                  (:Is%20Valid
                    (Variables|Default|SetOwnerController (Variables|Default|GetOwnerController)))
                  (:Is%20Not%20Valid
                    (bind _asbp_base_player_controller (Utilities|Casting|CastToBP_BasePlayerController (LocalVariables|GetInstigatorController)))
                    (Variables|Default|SetOwnerController _asbp_base_player_controller))))
              (:then_2
                (Utilities|IsValid (Variables|Default|GetOwnerController)
                  (:Is%20Valid
                    (Utilities|IsValid (Variables|Default|GetOwnerCharacter)
                      (:Is%20Valid
                        (Utilities|IsValid (Variables|/Game/BluePrints/Character/BP_BaseCharacter.BP_BaseCharacter_C|GetLagCompensation_Component (Variables|Default|GetOwnerCharacter))
                          (:Is%20Valid
                            (if (Pawn|IsLocallyControlled (Variables|Default|GetOwnerCharacter))
                              (Default|ShotgunServerScoreRequest (Variables|/Game/BluePrints/Character/BP_BaseCharacter.BP_BaseCharacter_C|GetLagCompensation_Component (Variables|Default|GetOwnerCharacter)) (LocalVariables|GetHitCharacters) (LocalVariables|GetStart) HitTargetsInput (- (Default|GetServerTime (Variables|Default|GetOwnerController)) (Variables|/Game/BluePrints/PlayerController/BP_BasePlayerController.BP_BasePlayerController_C|GetSingleTripTime (Variables|Default|GetOwnerController)))))))))))))))))))