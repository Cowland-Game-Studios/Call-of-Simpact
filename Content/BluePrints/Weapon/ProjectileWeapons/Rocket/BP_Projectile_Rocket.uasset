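; Rocket projectile Blueprint that deals explosion damage on impact.
; BeginPlay starts the inherited destroy timer and trail, and attaches a looping flight sound.
; Collision hits, except on the owner, call ExplodeDamage and spawn impact particles and sound.
; The rocket then hides its mesh, disables collision, and stops trail and loop sound instead of destroying itself immediately.
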(event OnComponentHit(CollisionBox)
  (params (HitComponent :type Primitive%20Component%20Object%20Reference) (OtherActor :type Actor%20Object%20Reference) (OtherComp :type Primitive%20Component%20Object%20Reference) (NormalImpulse :type Vector :default "0, 0, 0") (Hit :type Hit%20Result%20Structure%20%28by%20ref%29))
  ;[1 1 1] Rocket radial damage on hit
  (CallFunction|ApplyRadialDammageRocket OtherActor))

(event EventBeginPlay
  ;[1 1 1] Spawn Rocket Trail effect
  (CallFunction|StartDestroyTimer)
  (CallFunction|SpawnTrailSystem)
  (Utilities|IsValid (Variables|Sound|GetProjectileLoop)
    (:Is%20Valid
      (Utilities|IsValid (Variables|Sound|GetLoopingSoundAttenuation)
        (:Is%20Valid
          (bind _returnvalue (Audio|SpawnSoundAttached (Variables|Sound|GetProjectileLoop) (Variables|Transformation|GetRootComponent) "None" (Transformation|GetActorLocation) "0, 0, 0" "KeepWorldPosition" false 1.0 1.0 0.0 (Variables|Sound|GetLoopingSoundAttenuation) 0 false))
          (Variables|Sound|SetProjectileLoopComponent _returnvalue))))))

(event EventDestroyed
  ;[1 0.1229 0.3546] Don't delete
)

(fn ConstructionScript
  (|CallParentFunction))

(fn ApplyRadialDammageRocket
  (params (OtherActor :type Actor%20Object%20Reference))
  (bind _collisionbox (Variables|Default|GetCollisionBox))
  (bind _trailsystemcomponent (Variables|Default|GetTrailSystemComponent))
  (bind _projectilemesh (Variables|Default|GetProjectileMesh))
  (bind _projectileloopcomponent (Variables|Sound|GetProjectileLoopComponent))
  (Utilities|FlowControl|Sequence
    (:then_0
      (if (== OtherActor (Components|GetOwner))
        (return)))
    (:then_1
      ;[1 1 1] Apply explode damage
      (CallFunction|ExplodeDamage))
    (:then_2
      ;[1 1 1] Spawn sound and explision efects
      (CallFunction|SpawnRocketEffects))
    (:then_3
      ;[1 1 1] Hide mesh and disable collision
      (Utilities|IsValid _projectilemesh
        (:Is%20Valid
          (Rendering|SetVisibility _projectilemesh false false)
          (Utilities|IsValid _collisionbox
            (:Is%20Valid
              (Collision|SetCollisionEnabled _collisionbox "NoCollision"))))))
    (:then_4
      ;[1 1 1] Deactivate the particle
      (Utilities|IsValid _trailsystemcomponent
        (:Is%20Valid
          (Components|Activation|Deactivate _trailsystemcomponent))))
    (:then_5
      (if (and (Utilities|IsValid _projectileloopcomponent) (Audio|Components|Audio|IsPlaying _projectileloopcomponent))
        (Audio|Components|Audio|Stop _projectileloopcomponent)))))

(fn SpawnRocketEffects
  (bind _returnvalue (Transformation|GetActorTransform))
  (bind _impactparticles (Variables|Default|GetImpactParticles))
  (bind _impactsound (Variables|Default|GetImpactSound))
  (Utilities|FlowControl|Sequence
    (:then_0
      (Utilities|IsValid _impactparticles
        (:Is%20Valid
          (Effects|SpawnEmitteratLocation _impactparticles (.location _returnvalue) (.rotation _returnvalue) (.scale _returnvalue) false))))
    (:then_1
      (Utilities|IsValid _impactsound
        (:Is%20Valid
          (Audio|PlaySoundatLocation _impactsound (Transformation|GetActorLocation) "0, 0, 0" 1.0 1.0 0.0 0 0 0 0))))))