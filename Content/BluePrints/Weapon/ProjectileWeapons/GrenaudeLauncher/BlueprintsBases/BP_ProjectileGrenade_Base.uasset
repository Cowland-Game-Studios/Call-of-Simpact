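; Base Blueprint for grenade launcher projectiles that bounce and explode when destroyed.
; On BeginPlay it spawns a trail system and starts a destroy timer, and each bounce plays an optional sound at the grenade's location.
; Destruction applies explosion damage before calling the parent's Destroyed logic.
; The collision box hit event is deliberately kept empty and marked "Don't Delete", so hits trigger nothing in this graph.
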(event OnComponentHit(CollisionBox)
  (params (HitComponent :type Primitive%20Component%20Object%20Reference) (OtherActor :type Actor%20Object%20Reference) (OtherComp :type Primitive%20Component%20Object%20Reference) (NormalImpulse :type Vector :default "0, 0, 0") (Hit :type Hit%20Result%20Structure%20%28by%20ref%29))
  ;[1 0.02461 0.3495] Don't Delete
)

(event OnProjectileBounce(ProjectileMovement)
  (params (ImpactResult :type Hit%20Result%20Structure%20%28by%20ref%29) (ImpactVelocity :type Vector%20%28by%20ref%29 :default "0, 0, 0"))
  (bind _bouncesound (Variables|Default|GetBounceSound))
  ;[1 1 1] Bouncing Sound
  (Utilities|IsValid _bouncesound
    (:Is%20Valid
      (Audio|PlaySoundatLocation _bouncesound (Transformation|GetActorLocation) "0, 0, 0" 1.0 1.0 0.0 0 0 0 0))))

(event EventBeginPlay
  ;[1 1 1] Begin Play
  (CallFunction|SpawnTrailSystem)
  (CallFunction|StartDestroyTimer))

(event EventDestroyed
  ;[1 1 1] Destroyed
  (CallFunction|ExplodeDamage)
  (|CallParentFunction))

(fn ConstructionScript
  (|CallParentFunction))