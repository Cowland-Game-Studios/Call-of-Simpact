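; Base multiplayer game mode that runs match flow, elimination scoring and respawns.
; Tick counts down warmup, match and cooldown before restarting, and state changes gather controllers from player states to notify them.
; PlayerEliminated resolves player or AI player states, updates score, deaths and top-scorer lead multicasts, then broadcasts the elimination.
; RequestRespawn restarts players at random PlayerStarts, and CalculateDamage passes base damage through unchanged.
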(event EventBeginPlay
  ;[1 1 1] Level Starting Time
  (Variables|Time|SetLevelStartingTime (Utilities|Time|GetTimeSeconds)))

(event EventTick
  (params (DeltaSeconds :type Float%20%28single-precision%29))
  (bind _returnvalue (Class|GameMode|GetMatchState))
  (bind _returnvalue_2 (Utilities|Time|GetTimeSeconds))
  (bind _warmuptime (Variables|Time|GetWarmupTime))
  (bind _matchtime (Variables|Time|GetMatchTime))
  (bind _levelstartingtime (Variables|Time|GetLevelStartingTime))
  (bind _returnvalue_3 (+ _warmuptime _matchtime))
  (bind _returnvalue_4 (- _returnvalue_3 _returnvalue_2))
  (bind _returnvalue_5 (+ _returnvalue_4 _levelstartingtime))
  ;[1 1 1] Warmup Time before starting Game
  (if (== _returnvalue "WaitingToStart")
    (bind _output_get (Variables|Time|SetCountdownTime (+ (- (Variables|Time|GetWarmupTime) (Utilities|Time|GetTimeSeconds)) (Variables|Time|GetLevelStartingTime))))
    (if (<= _output_get 0.0)
      (Class|GameMode|StartMatch))
    (elif (== _returnvalue "InProgress")
      (bind _output_get_2 (Variables|Time|SetCountdownTime _returnvalue_5))
      (if (<= _output_get_2 0.0)
        (Class|BlasterMapGamemode|SetNewMatchState "Cooldown"))
      (elif (== _returnvalue "Cooldown")
        (bind _output_get_3 (Variables|Time|SetCountdownTime (+ _returnvalue_5 (Variables|Time|GetCooldownTime))))
        (if (<= _output_get_3 0.0)
          (Class|GameMode|RestartGame))))))

(event EventOnSetMatchState
  (params (NewState :type Name :default "None"))
  ;[1 1 1] On Match State Set
  (CallFunction|OnMatchStateSetFunctionEvent NewState))

(fn ConstructionScript)

(fn PlayerEliminated
  (params (ElimmedCharacter :type BP%20Base%20Character%20Object%20Reference) (VictimController :type BP%20Base%20Player%20Controller%20Object%20Reference) (AttackerController :type BP%20Base%20Player%20Controller%20Object%20Reference) (AI_AttackerController :type ALS%20AI%20Controller%20Object%20Reference) (AI_VictimController :type ALS%20AI%20Controller%20Object%20Reference))
  (Variables|/Game/BluePrints/Character/BP_BaseCharacter.BP_BaseCharacter_C|SetDead ElimmedCharacter true)
  (Utilities|FlowControl|Sequence
    (:then_0
      ;[1 1 1] Set Attacker and victim Player states
      (Utilities|IsValid AttackerController
        (:Is%20Valid
          (bind _asbp_base_player_state (Utilities|Casting|CastToBP_BasePlayerState (Variables|/Script/Engine.Controller|GetPlayerState AttackerController)))
          (LocalVariables|SetAttackerPlayerState _asbp_base_player_state))
        (:Is%20Not%20Valid
          ;;[0.1354 1 0.5504] Attacker is an AI
          (Utilities|IsValid AI_AttackerController
            (:Is%20Valid
              (bind _asbp_base_player_state_2 (Utilities|Casting|CastToBP_BasePlayerState (Variables|/Script/Engine.Controller|GetPlayerState AI_AttackerController)))
              (LocalVariables|SetAttackerPlayerState _asbp_base_player_state_2))
            (:Is%20Not%20Valid
              (LocalVariables|SetAttackerPlayerState 0))))))
    (:then_1
      (Utilities|IsValid VictimController
        (:Is%20Valid
          (bind _asbp_base_player_state_3 (Utilities|Casting|CastToBP_BasePlayerState (Variables|/Script/Engine.Controller|GetPlayerState VictimController)))
          (LocalVariables|SetVictimPlayerState _asbp_base_player_state_3))
        (:Is%20Not%20Valid
          (bind _asbp_base_player_state_4 (Utilities|Casting|CastToBP_BasePlayerState (Variables|/Script/Engine.Controller|GetPlayerState AI_VictimController)))
          (bind _output_get (LocalVariables|SetVictimPlayerState _asbp_base_player_state_4))
          (Development|PrintString (Utilities|GetDisplayName _output_get) true true "(R=0.783258,G=0.192708,B=1.000000,A=1.000000)" 1e+01))))
    (:then_2
      ;[1 1 1] Set Game state
      (Utilities|IsValid (Variables|Default|GetBaseGameState)
        (:Is%20Valid
          (Variables|Default|SetBaseGameState (Variables|Default|GetBaseGameState)))
        (:Is%20Not%20Valid
          (bind _asbp_base_game_state (Utilities|Casting|CastToBP_BaseGameState (Game|GetGameState)))
          (Variables|Default|SetBaseGameState _asbp_base_game_state))))
    (:then_3
      ;[1 1 1] Add Score
      (for _array_element (Variables|/Game/BluePrints/GameState/BP_BaseGameState.BP_BaseGameState_C|GetTopScoringPlayers (Variables|Default|GetBaseGameState))
        (Utilities|Array|Add (LocalVariables|GetPlayersCurrentyInTheLead) _array_element))
      (if (Math|Boolean|ANDBoolean (Utilities|IsValid (LocalVariables|GetAttackerPlayerState)) (!= (LocalVariables|GetAttackerPlayerState) (LocalVariables|GetVictimPlayerState)) (Utilities|IsValid (Variables|Default|GetBaseGameState)))
        (Default|AddtoScore (LocalVariables|GetAttackerPlayerState) 1.0)
        (Default|UpdateTopScore (Variables|Default|GetBaseGameState) (LocalVariables|GetAttackerPlayerState))
        (Utilities|FlowControl|Sequence
          (:then_0
            (if (Utilities|Array|ContainsItem (Variables|/Game/BluePrints/GameState/BP_BaseGameState.BP_BaseGameState_C|GetTopScoringPlayers (Variables|Default|GetBaseGameState)) (LocalVariables|GetAttackerPlayerState))
              (bind _asbp_base_character (Utilities|Casting|CastToBP_BaseCharacter (PlayerState|GetPawn (LocalVariables|GetAttackerPlayerState))))
              (bind _output_get_2 (LocalVariables|SetLeader _asbp_base_character))
              (Default|MultiCastGainedtheLead _output_get_2)))
          (:then_1
            (for _index (range 0 (- (Utilities|Array|Length (LocalVariables|GetPlayersCurrentyInTheLead)) 1))
              (if (not (Utilities|Array|ContainsItem (Variables|/Game/BluePrints/GameState/BP_BaseGameState.BP_BaseGameState_C|GetTopScoringPlayers (Variables|Default|GetBaseGameState)) (Utilities|Array|Get(acopy) (LocalVariables|GetPlayersCurrentyInTheLead) _index)))
                (bind _asbp_base_character_2 (Utilities|Casting|CastToBP_BaseCharacter (PlayerState|GetPawn (Utilities|Array|Get(acopy) (LocalVariables|GetPlayersCurrentyInTheLead) _index))))
                (bind _output_get_3 (LocalVariables|SetLoser _asbp_base_character_2))
                (Utilities|IsValid _output_get_3
                  (:Is%20Valid
                    (Default|MulticastLosttheLead _output_get_3)))))))
        (else
          (Development|PrintString "False" true true "(R=1.000000,G=0.050654,B=0.100414,A=1.000000)" 1e+01))))
    (:then_4
      ;[1 1 1] Is not AI
      (if (Class|Pawn|IsControlled ElimmedCharacter)
        ;[1 1 1] Add to deaths
        (Default|AddtoDeaths (LocalVariables|GetVictimPlayerState) 1)))
    (:then_5
      ;[1 1 1] Elimination
      (Utilities|IsValid ElimmedCharacter
        (:Is%20Valid
          (Default|Elim ElimmedCharacter))))
    (:then_6
      ;[1 1 1] ElimAnnouncement
      (for _index_2 (range 0 (- (Class|GameplayStatics|GetNumPlayerControllers) 1))
        (bind _asbp_base_player_controller (Utilities|Casting|CastToBP_BasePlayerController (Game|GetPlayerController _index_2)))
        (bind _output_get_4 (LocalVariables|SetBasePlayerController _asbp_base_player_controller))
        (Utilities|IsValid _output_get_4
          (:Is%20Valid
            (Utilities|IsValid (LocalVariables|GetAttackerPlayerState)
              (:Is%20Valid
                (Utilities|IsValid (LocalVariables|GetVictimPlayerState)
                  (:Is%20Valid
                    (Default|BroadcastElim (LocalVariables|GetBasePlayerController) (LocalVariables|GetAttackerPlayerState) (LocalVariables|GetVictimPlayerState))))))))))))

(fn RequestRespawn
  (params (ElimmedCharacter :type BP%20Base%20Character%20Object%20Reference) (ElimmedController :type BP%20Base%20Player%20Controller%20Object%20Reference))
  (Utilities|FlowControl|Sequence
    (:then_0
      ;[1 1 1] Destroy Player
      (Utilities|IsValid ElimmedCharacter
        (:Is%20Valid
          (Class|VectortoRotator|ResetPlayer ElimmedCharacter))))
    (:then_1
      ;[1 1 1] Respawn
      (Utilities|IsValid ElimmedController
        (:Is%20Valid
          (bind _outactors (Actor|GetAllActorsOfClass "/Script/Engine.PlayerStart"))
          (bind _output_get (LocalVariables|SetPlayerStarts _outactors))
          (LocalVariables|SetSelection (Math|Random|RandomInteger (- (Utilities|Array|Length _output_get) 1)))
          (Class|GameModeBase|RestartPlayeratPlayerStart ElimmedController (Utilities|Array|Get(acopy) (LocalVariables|GetPlayerStarts) (LocalVariables|GetSelection))))))))

(fn SendControllerstoGameMode
  (params (MatchStateFunc :type Name))
  (for _index (range 0 (Class|GameplayStatics|GetNumPlayerStates))
    (bind _asbp_base_player_state (Utilities|Casting|CastToBP_BasePlayerState (Game|GetPlayerState _index)))
    (Default|SetControllerinPlayerState _asbp_base_player_state)
    (Utilities|IsValid (Variables|/Game/BluePrints/PlayerState/BP_BasePlayerState.BP_BasePlayerState_C|GetController _asbp_base_player_state)
      (:Is%20Valid
        (Utilities|Array|AddUnique (Variables|Default|GetPlayerControllers) (Variables|/Game/BluePrints/PlayerState/BP_BasePlayerState.BP_BasePlayerState_C|GetController _asbp_base_player_state))))))

(fn OnMatchStateSetFunctionEvent
  (params (Match%20StateFunc :type Name))
  (bind _playercontrollers (Variables|Default|GetPlayerControllers))
  (Utilities|FlowControl|Sequence
    (:then_0
      ;[1 1 1] Initialise Controllers
      (CallFunction|SendControllerstoGameMode Match%20StateFunc))
    (:then_1
      (if (Utilities|Array|IsNotEmpty _playercontrollers)
        (for _array_element _playercontrollers
          (bind _output_get (LocalVariables|SetBasePlayer _array_element))
          (Utilities|IsValid _output_get
            (:Is%20Valid
              (Default|OnMatchStateSet (LocalVariables|GetBasePlayer) (Class|GameMode|GetMatchState) (Variables|Teams|GetTeamsMatch)))))))))

(fn CalculateDamage
  (params (AttackerController :type Controller%20Object%20Reference) (VictimController :type Controller%20Object%20Reference) (BaseDamage :type Float%20%28double-precision%29))
  (return BaseDamage))