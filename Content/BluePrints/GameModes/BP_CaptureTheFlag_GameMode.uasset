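; Capture the Flag game mode that awards a team score when a flag is captured in a zone.
; FlagCaptured gets BP_BaseGameState and calls the Blue or Red team scoring function based on the capture zone's team.
; It computes whether the flag and zone teams differ, but scoring does not check that result.
; Player elimination forwards to the parent implementation, omitting the AI controller arguments.
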(event EventBeginPlay
  (|CallParentFunction) ; This node is disabled and will not be called.\nDrag off pins to build functionality.
)

(event EventTick
  (params (DeltaSeconds :type Float%20%28single-precision%29))
  (|CallParentFunction DeltaSeconds) ; This node is disabled and will not be called.\nDrag off pins to build functionality.
)

(fn ConstructionScript
  (|CallParentFunction))

(fn PlayerEliminated
  (params (ElimmedCharacter :type BP%20Base%20Character%20Object%20Reference) (VictimController :type BP%20Base%20Player%20Controller%20Object%20Reference) (AttackerController :type BP%20Base%20Player%20Controller%20Object%20Reference) (AI_AttackerController :type ALS%20AI%20Controller%20Object%20Reference) (AI_VictimController :type ALS%20AI%20Controller%20Object%20Reference))
  (|CallParentFunction ElimmedCharacter VictimController AttackerController 0 0))

(fn FlagCaptured
  (params (Flag :type BP%20Flag%20Base%20Object%20Reference) (Zone :type Flag%20Zone%20Base%20Object%20Reference))
  (LocalVariables|SetValidCapture (Utilities|Enum|NotEqual(Enum) (Variables|/Game/BluePrints/Weapon/BlueprintBases/BP_Weapon_Base.BP_Weapon_Base_C|GetFlagTeam Flag) (Variables|/Game/BluePrints/Flag/FlagZones/FlagZone_Base.FlagZone_Base_C|GetTeam Zone)))
  (bind _asbp_base_game_state (Utilities|Casting|CastToBP_BaseGameState (Game|GetGameState)))
  (bind _output_get (LocalVariables|SetBGameState _asbp_base_game_state))
  (Utilities|IsValid _output_get
    (:Is%20Valid
      (Utilities|FlowControl|Sequence
        (:then_0
          (if (Utilities|Enum|Equal(Enum) (Variables|/Game/BluePrints/Flag/FlagZones/FlagZone_Base.FlagZone_Base_C|GetTeam Zone) "NewEnumerator0")
            (Default|BlueTeamScores (LocalVariables|GetBGameState))))
        (:then_1
          (if (Utilities|Enum|Equal(Enum) (Variables|/Game/BluePrints/Flag/FlagZones/FlagZone_Base.FlagZone_Base_C|GetTeam Zone) "NewEnumerator1")
            (Default|RedTeamScores (LocalVariables|GetBGameState))))))))