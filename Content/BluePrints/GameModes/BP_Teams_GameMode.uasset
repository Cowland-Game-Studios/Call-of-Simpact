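; Team-match game mode that splits players into Red and Blue teams, filters friendly fire and awards team points for eliminations.
; Unassigned players join the smaller team (Red on ties) on login or when starting after the match has begun, and leave the GameState rosters on logout.
; Damage between teammates is zeroed unless Teamkill is on, while self-damage still applies.
; Eliminations score for the attacker's team through BP_BaseGameState, except in capture-the-flag modes.
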(event EventPostLogin
  (params (NewPlayer :type Player%20Controller%20Object%20Reference))
  (|CallParentFunction NewPlayer)
  (CallFunction|PostLoginSortTeam NewPlayer))

(event EventOnLogout
  (params (ExitingController :type Controller%20Object%20Reference))
  (|CallParentFunction ExitingController)
  (CallFunction|OnLogout ExitingController))

(event EventHandleStartingNewPlayer
  (params (NewPlayer :type Player%20Controller%20Object%20Reference))
  (|CallParentFunction NewPlayer)
  (CallFunction|HandleMatchStart))

(fn ConstructionScript
  (|CallParentFunction)
  (Variables|Default|SetTeamsMatch true))

(fn SendControllerstoGameMode
  (params (MatchStateFunc :type Name :default "None"))
  (|CallParentFunction MatchStateFunc))

(fn HandleMatchStart
  (if (Class|GameModeBase|HasMatchStarted)
    (bind _asbp_base_game_state (Utilities|Casting|CastToBP_BaseGameState (Game|GetGameState)))
    (bind _output_get (LocalVariables|SetBGameState _asbp_base_game_state))
    (Utilities|IsValid _output_get
      (:Is%20Valid
        (for _array_element (Variables|/Script/Engine.GameStateBase|GetPlayerArray _output_get)
          (bind _asbp_base_player_state (Utilities|Casting|CastToBP_BasePlayerState _array_element))
          (bind _output_get_2 (LocalVariables|SetBPState _asbp_base_player_state))
          (Utilities|IsValid _output_get_2
            (:Is%20Valid
              (if (Utilities|Enum|Equal(Enum) (Variables|/Game/BluePrints/PlayerState/BP_BasePlayerState.BP_BasePlayerState_C|GetTeam _output_get_2) "NewEnumerator2")
                (if (>= (Utilities|Array|Length (Variables|/Game/BluePrints/GameState/BP_BaseGameState.BP_BaseGameState_C|GetBlueTeam (LocalVariables|GetBGameState))) (Utilities|Array|Length (Variables|/Game/BluePrints/GameState/BP_BaseGameState.BP_BaseGameState_C|GetRedTeam (LocalVariables|GetBGameState))))
                  (Utilities|Array|AddUnique (Variables|/Game/BluePrints/GameState/BP_BaseGameState.BP_BaseGameState_C|GetRedTeam (LocalVariables|GetBGameState)) (LocalVariables|GetBPState))
                  (Default|SetTeam (LocalVariables|GetBPState) "NewEnumerator1")
                  (else
                    (Utilities|Array|AddUnique (Variables|/Game/BluePrints/GameState/BP_BaseGameState.BP_BaseGameState_C|GetBlueTeam (LocalVariables|GetBGameState)) (LocalVariables|GetBPState))
                    (Default|SetTeam (LocalVariables|GetBPState) "NewEnumerator0")))))))))))

(fn PostLoginSortTeam
  (params (New%20Player :type Player%20Controller%20Object%20Reference))
  (bind _asbp_base_game_state (Utilities|Casting|CastToBP_BaseGameState (Game|GetGameState)))
  (bind _output_get (LocalVariables|SetBGameState _asbp_base_game_state))
  (Utilities|IsValid _output_get
    (:Is%20Valid
      (bind _asbp_base_player_state (Utilities|Casting|CastToBP_BasePlayerState (Variables|/Script/Engine.Controller|GetPlayerState New%20Player)))
      (bind _output_get_2 (LocalVariables|SetBPState _asbp_base_player_state))
      (Utilities|IsValid _output_get_2
        (:Is%20Valid
          (if (Utilities|Enum|Equal(Enum) (Variables|/Game/BluePrints/PlayerState/BP_BasePlayerState.BP_BasePlayerState_C|GetTeam _output_get_2) "NewEnumerator2")
            (if (>= (Utilities|Array|Length (Variables|/Game/BluePrints/GameState/BP_BaseGameState.BP_BaseGameState_C|GetBlueTeam (LocalVariables|GetBGameState))) (Utilities|Array|Length (Variables|/Game/BluePrints/GameState/BP_BaseGameState.BP_BaseGameState_C|GetRedTeam (LocalVariables|GetBGameState))))
              (Utilities|Array|AddUnique (Variables|/Game/BluePrints/GameState/BP_BaseGameState.BP_BaseGameState_C|GetRedTeam (LocalVariables|GetBGameState)) (LocalVariables|GetBPState))
              (Default|SetTeam (LocalVariables|GetBPState) "NewEnumerator1")
              (else
                (Utilities|Array|AddUnique (Variables|/Game/BluePrints/GameState/BP_BaseGameState.BP_BaseGameState_C|GetBlueTeam (LocalVariables|GetBGameState)) (LocalVariables|GetBPState))
                (Default|SetTeam (LocalVariables|GetBPState) "NewEnumerator0")))))))))

(fn OnLogout
  (params (ExitingPlayer :type Controller%20Object%20Reference))
  (bind _asbp_base_game_state (Utilities|Casting|CastToBP_BaseGameState (Game|GetGameState)))
  (bind _output_get (LocalVariables|SetBGameState _asbp_base_game_state))
  (bind _asbp_base_player_state (Utilities|Casting|CastToBP_BasePlayerState (Variables|/Script/Engine.Controller|GetPlayerState ExitingPlayer)))
  (bind _output_get_2 (LocalVariables|SetBPState _asbp_base_player_state))
  (Utilities|IsValid _output_get_2
    (:Is%20Valid
      (Utilities|IsValid _output_get
        (:Is%20Valid
          (Utilities|FlowControl|Sequence
            (:then_0
              (if (Utilities|Array|ContainsItem (Variables|/Game/BluePrints/GameState/BP_BaseGameState.BP_BaseGameState_C|GetRedTeam (LocalVariables|GetBGameState)) (LocalVariables|GetBPState))
                (Utilities|Array|RemoveItem (Variables|/Game/BluePrints/GameState/BP_BaseGameState.BP_BaseGameState_C|GetRedTeam (LocalVariables|GetBGameState)) (LocalVariables|GetBPState))))
            (:then_1
              (if (Utilities|Array|ContainsItem (Variables|/Game/BluePrints/GameState/BP_BaseGameState.BP_BaseGameState_C|GetBlueTeam (LocalVariables|GetBGameState)) (LocalVariables|GetBPState))
                (Utilities|Array|RemoveItem (Variables|/Game/BluePrints/GameState/BP_BaseGameState.BP_BaseGameState_C|GetBlueTeam (LocalVariables|GetBGameState)) (LocalVariables|GetBPState))))))))))

(fn CalculateDamage
  (params (AttackerController :type Controller%20Object%20Reference) (VictimController :type Controller%20Object%20Reference) (BaseDamage :type Float%20%28double-precision%29))
  (if (Variables|Default|GetTeamkill)
    (return BaseDamage)
    (else
      (Utilities|FlowControl|Sequence
        (:then_0
          (bind _asbp_base_player_state (Utilities|Casting|CastToBP_BasePlayerState (Variables|/Script/Engine.Controller|GetPlayerState AttackerController)))
          (bind _output_get (LocalVariables|SetAttackerBState _asbp_base_player_state))
          (Utilities|IsValid _output_get
            (:Is%20Not%20Valid
              (return BaseDamage))))
        (:then_1
          (bind _asbp_base_player_state_2 (Utilities|Casting|CastToBP_BasePlayerState (Variables|/Script/Engine.Controller|GetPlayerState VictimController)))
          (bind _output_get_2 (LocalVariables|SetVictimBState _asbp_base_player_state_2))
          (Utilities|IsValid _output_get_2
            (:Is%20Not%20Valid
              (return BaseDamage))))
        (:then_2
          (Utilities|IsValid (LocalVariables|GetVictimBState)
            (:Is%20Valid
              (if (== (LocalVariables|GetAttackerBState) (LocalVariables|GetVictimBState))
                (return BaseDamage)))))
        (:then_3
          (Utilities|IsValid (LocalVariables|GetVictimBState)
            (:Is%20Valid
              (if (Utilities|Enum|Equal(Enum) (Variables|/Game/BluePrints/PlayerState/BP_BasePlayerState.BP_BasePlayerState_C|GetTeam (LocalVariables|GetAttackerBState)) (Variables|/Game/BluePrints/PlayerState/BP_BasePlayerState.BP_BasePlayerState_C|GetTeam (LocalVariables|GetVictimBState)))
                (return 0.0)))))
        (:then_4
          (return BaseDamage))))))

(fn PlayerEliminated
  (params (ElimmedCharacter :type BP%20Base%20Character%20Object%20Reference) (VictimController :type BP%20Base%20Player%20Controller%20Object%20Reference) (AttackerController :type BP%20Base%20Player%20Controller%20Object%20Reference) (AI_AttackerController :type ALS%20AI%20Controller%20Object%20Reference) (AI_VictimController :type ALS%20AI%20Controller%20Object%20Reference))
  (|CallParentFunction ElimmedCharacter VictimController AttackerController 0 0)
  (if (not (Variables|Default|GetIsCaptureFlagGameMode))
    (Utilities|FlowControl|Sequence
      (:then_0
        (bind _asbp_base_game_state (Utilities|Casting|CastToBP_BaseGameState (Game|GetGameState)))
        (LocalVariables|SetBGameState _asbp_base_game_state))
      (:then_1
        (Utilities|IsValid AttackerController
          (:Is%20Valid
            (bind _asbp_base_player_state (Utilities|Casting|CastToBP_BasePlayerState (Variables|/Script/Engine.Controller|GetPlayerState AttackerController)))
            (LocalVariables|SetAttackerPlayerState _asbp_base_player_state))
          (:Is%20Not%20Valid
            (LocalVariables|SetAttackerPlayerState 0))))
      (:then_2
        (Utilities|IsValid (LocalVariables|GetBGameState)
          (:Is%20Valid
            (Utilities|IsValid (LocalVariables|GetAttackerPlayerState)
              (:Is%20Valid
                (Utilities|FlowControl|Sequence
                  (:then_0
                    (if (Utilities|Enum|Equal(Enum) (Variables|/Game/BluePrints/PlayerState/BP_BasePlayerState.BP_BasePlayerState_C|GetTeam (LocalVariables|GetAttackerPlayerState)) "NewEnumerator0")
                      (Default|BlueTeamScores (LocalVariables|GetBGameState))))
                  (:then_1
                    (if (Utilities|Enum|Equal(Enum) (Variables|/Game/BluePrints/PlayerState/BP_BasePlayerState.BP_BasePlayerState_C|GetTeam (LocalVariables|GetAttackerPlayerState)) "NewEnumerator1")
                      (Default|RedTeamScores (LocalVariables|GetBGameState)))))))))))))