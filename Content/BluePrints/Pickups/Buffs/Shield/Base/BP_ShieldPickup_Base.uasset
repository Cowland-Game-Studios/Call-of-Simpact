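; Base shield pickup that grants a timed shield buff to an overlapping BP_BaseCharacter.
; Its sphere overlap calls Overlapping, which passes ShieldAmount and ShieldTime to the character's BuffComponent.
; A character already at MaxShield exits early, leaving the pickup in place.
; Otherwise a Sequence destroys the pickup, even when the cast fails or the BuffComponent is invalid.
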(event OnComponentBeginOverlap(OverlapSphere)
  (params (OverlappedComponent :type Primitive%20Component%20Object%20Reference) (OtherActor :type Actor%20Object%20Reference) (OtherComp :type Primitive%20Component%20Object%20Reference) (OtherBodyIndex :type Integer) (bFromSweep :type Boolean) (SweepResult :type Hit%20Result%20Structure%20%28by%20ref%29))
  (CallFunction|Overlapping OtherActor))

(event EventBeginPlay
  (|CallParentFunction) ; This node is disabled and will not be called.\nDrag off pins to build functionality.
)

(event Collision|EventActorBeginOverlap
  (params (OtherActor :type Actor%20Object%20Reference))
  (|CallParentFunction OtherActor) ; This node is disabled and will not be called.\nDrag off pins to build functionality.
)

(event EventTick
  (params (DeltaSeconds :type Float%20%28single-precision%29))
  (|CallParentFunction DeltaSeconds) ; This node is disabled and will not be called.\nDrag off pins to build functionality.
)

(fn ConstructionScript
  (|CallParentFunction))

(fn Overlapping
  (params (InputPin :type Actor%20Object%20Reference))
  (Utilities|FlowControl|Sequence
    (:then_0
      (bind _asbp_base_character (Utilities|Casting|CastToBP_BaseCharacter InputPin))
      (bind _output_get (Variables|Default|SetBaseCharacter _asbp_base_character))
      (if (== (Variables|/Game/BluePrints/Character/BP_BaseCharacter.BP_BaseCharacter_C|GetShield _output_get) (Variables|/Game/BluePrints/Character/BP_BaseCharacter.BP_BaseCharacter_C|GetMaxShield _output_get))
        (return)
        (else
          (Utilities|IsValid (Variables|/Game/BluePrints/Character/BP_BaseCharacter.BP_BaseCharacter_C|GetBuffComponent _output_get)
            (:Is%20Valid
              (Default|Shield (Variables|/Game/BluePrints/Character/BP_BaseCharacter.BP_BaseCharacter_C|GetBuffComponent _output_get) (Variables|Default|GetShieldAmount) (Variables|Default|GetShieldTime)))))))
    (:then_1
      (Actor|DestroyActor))))