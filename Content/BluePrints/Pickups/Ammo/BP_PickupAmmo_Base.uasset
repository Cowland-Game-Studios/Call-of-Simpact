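; Base ammo pickup actor that grants ammo of a set weapon type to an overlapping character.
; On BeginPlay it writes the weapon type's enum name into its WBP_AmmoName widget.
; A sphere overlap passes the type and amount to the BP_BaseCharacter's Combat component through PickUpAmmo.
; A Sequence then destroys the pickup on any overlap, even when the other actor is not a character.
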(event OnComponentBeginOverlap(OverlapSphere)
  (params (OverlappedComponent :type Primitive%20Component%20Object%20Reference) (OtherActor :type Actor%20Object%20Reference) (OtherComp :type Primitive%20Component%20Object%20Reference) (OtherBodyIndex :type Integer) (bFromSweep :type Boolean) (SweepResult :type Hit%20Result%20Structure%20%28by%20ref%29))
  (Utilities|FlowControl|Sequence
    (:then_0
      (bind _asbp_base_character (Utilities|Casting|CastToBP_BaseCharacter OtherActor))
      (bind _output_get (Variables|Default|SetBaseCharacter _asbp_base_character))
      (Utilities|IsValid _output_get
        (:Is%20Valid
          (Utilities|IsValid (Variables|/Game/AdvancedLocomotionV4/Blueprints/CharacterLogic/ALS_AnimMan_CharacterBP.ALS_AnimMan_CharacterBP_C|GetCombat _output_get)
            (:Is%20Valid
              (Default|PickUpAmmo (Variables|/Game/AdvancedLocomotionV4/Blueprints/CharacterLogic/ALS_AnimMan_CharacterBP.ALS_AnimMan_CharacterBP_C|GetCombat _output_get) (Variables|Default|GetWeaponType) (Variables|Default|GetAmmoAmount)))))))
    (:then_1
      (Actor|DestroyActor))))

(event EventBeginPlay
  (bind _pickup_ammo_widget (Variables|Default|GetPickUp%20Ammo%20Widget))
  (|CallParentFunction)
  (Utilities|IsValid _pickup_ammo_widget
    (:Is%20Valid
      (bind _aswbp_ammo_name (Utilities|Casting|CastToWBP_AmmoName (UserInterface|GetWidget _pickup_ammo_widget)))
      (Rendering|Components|TextRender|SetText (Variables|/Game/BluePrints/HUD/WBP_AmmoName.WBP_AmmoName_C|GetAmmoType _aswbp_ammo_name) (Utilities|Text|ToText(String) (Utilities|String|EnumtoString (Variables|Default|GetWeaponType)))))))

(event Collision|EventActorBeginOverlap
  (params (OtherActor :type Actor%20Object%20Reference))
  (|CallParentFunction OtherActor) ; This node is disabled and will not be called.\nDrag off pins to build functionality.
)

(event EventTick
  (params (DeltaSeconds :type Float%20%28single-precision%29))
  (|CallParentFunction DeltaSeconds) ; This node is disabled and will not be called.\nDrag off pins to build functionality.
)

(fn ConstructionScript
  (|CallParentFunction))