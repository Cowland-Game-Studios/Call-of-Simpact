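; BP_Flag_Base is the base carryable flag, built on weapon-style pickup components and state.
; It caches its spawn transform at BeginPlay and turns off custom depth at construction.
; OnEquipped hides the pickup widget, disables the pickup sphere and mesh physics, and clears custom depth.
; ResetFlag clears the carrying character's flag state, then on authority detaches the flag, restores pickup overlap and teleports it home, provided the owner cast succeeds.
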(event EventBeginPlay
  (|CallParentFunction)
  (Variables|Default|SetInitialLocation (Transformation|GetActorTransform)))

(fn ConstructionScript
  (|CallParentFunction)
  (CallFunction|AddCustomDepth false))

(fn ResetFlag
  (bind _area_sphere (Variables|Default|GetArea%20Sphere))
  (Utilities|FlowControl|Sequence
    (:then_0
      (bind _asbp_base_character (Utilities|Casting|CastToBP_BaseCharacter (Components|GetOwner)))
      (bind _output_get (LocalVariables|SetFlagBearer _asbp_base_character))
      (Default|SetHoldingtheFlag _output_get false)
      (Default|ResetCharacterFlag (Variables|/Game/AdvancedLocomotionV4/Blueprints/CharacterLogic/ALS_AnimMan_CharacterBP.ALS_AnimMan_CharacterBP_C|GetCombat _output_get))
      (Variables|/Game/BluePrints/Character/BP_BaseCharacter.BP_BaseCharacter_C|SetOverlappingWeapon _output_get 0))
    (:then_1
      (if (not (Ability|HasAuthority))
        (return)
        (else
          (Transformation|DetachFromComponent (Variables|Default|GetWeapon%20Mesh) "KeepWorld" "KeepWorld" "KeepWorld" false)
          (Actor|SetOwner 0)
          (Collision|SetCollisionEnabled (Variables|Default|GetArea%20Sphere) "QueryAndPhysics")
          (Variables|Default|SetWeaponStateN "NewEnumerator0")
          (Collision|SetCollisionEnabled _area_sphere "QueryAndPhysics")
          (Collision|SetCollisionResponsetoChannel _area_sphere "ECC_Pawn" "ECR_Overlap")
          (Variables|Default|SetOwnerRep 0)
          (Variables|Default|SetOwnerCharacter 0)
          (Variables|Default|SetOwnerController 0)
          (Transformation|SetActorTransform (Variables|Default|GetInitialLocation) false true))))))

(fn OnEquipped
  (bind _weapon_mesh (Variables|Default|GetWeapon%20Mesh))
  (Utilities|FlowControl|Sequence
    (:then_0
      ;[1 1 1] Equipped Weapon
      (CallFunction|ShowPickUpWidget false)
      (Collision|SetCollisionEnabled (Variables|Default|GetArea%20Sphere) "NoCollision")
      (Physics|SetSimulatePhysics _weapon_mesh false)
      (Physics|SetEnableGravity _weapon_mesh false)
      (Collision|SetCollisionEnabled _weapon_mesh "QueryOnly")
      (Collision|SetCollisionResponsetoChannel _weapon_mesh "ECC_WorldDynamic" "ECR_Overlap"))
    (:then_1
      (CallFunction|AddCustomDepth false))))