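; BP_Objective is an objective marker that registers its position with the player's compass.
; On BeginPlay it gets player 0's BP_BasePlayerController and, if the HUD's compass objective panel is valid, adds a new WB_ObjectivePoint widget to it.
; It then stores its location and that widget in the controller's NavPoints map.
; The location is captured once, with no updates or removal here.
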(event EventBeginPlay
  (Utilities|FlowControl|Sequence
    (:then_0
      ;[1 1 1] Player controller
      (bind _asbp_base_player_controller (Utilities|Casting|CastToBP_BasePlayerController (Game|GetPlayerController 0)))
      (Variables|Default|SetPlayerController _asbp_base_player_controller))
    (:then_1
      (Utilities|IsValid (Variables|/Game/BluePrints/PlayerController/BP_BasePlayerController.BP_BasePlayerController_C|GetBaseHUD (Variables|Default|GetPlayerController))
        (:Is%20Valid
          (Utilities|IsValid (Variables|/Game/BluePrints/HUD/BaseHUD.BaseHUD_C|GetCharacterOverlay (Variables|/Game/BluePrints/PlayerController/BP_BasePlayerController.BP_BasePlayerController_C|GetBaseHUD (Variables|Default|GetPlayerController)))
            (:Is%20Valid
              (Utilities|IsValid (Variables|/Game/BluePrints/HUD/WBP_CharacterOverlay.WBP_CharacterOverlay_C|GetWB_Compass (Variables|/Game/BluePrints/HUD/BaseHUD.BaseHUD_C|GetCharacterOverlay (Variables|/Game/BluePrints/PlayerController/BP_BasePlayerController.BP_BasePlayerController_C|GetBaseHUD (Variables|Default|GetPlayerController))))
                (:Is%20Valid
                  (Utilities|IsValid (Variables|/Game/BluePrints/HUD/WB_Compass.WB_Compass_C|GetObjectivePanel (Variables|/Game/BluePrints/HUD/WBP_CharacterOverlay.WBP_CharacterOverlay_C|GetWB_Compass (Variables|/Game/BluePrints/HUD/BaseHUD.BaseHUD_C|GetCharacterOverlay (Variables|/Game/BluePrints/PlayerController/BP_BasePlayerController.BP_BasePlayerController_C|GetBaseHUD (Variables|Default|GetPlayerController)))))
                    (:Is%20Valid
                      ;[1 1 1] Store position and icon widget
                      (bind _returnvalue (UserInterface|CreateWidget "/Game/BluePrints/HUD/WB_ObjectivePoint.WB_ObjectivePoint_C" (Variables|Default|GetPlayerController)))
                      (Widget|Panel|AddChild (Variables|/Game/BluePrints/HUD/WB_Compass.WB_Compass_C|GetObjectivePanel (Variables|/Game/BluePrints/HUD/WBP_CharacterOverlay.WBP_CharacterOverlay_C|GetWB_Compass (Variables|/Game/BluePrints/HUD/BaseHUD.BaseHUD_C|GetCharacterOverlay (Variables|/Game/BluePrints/PlayerController/BP_BasePlayerController.BP_BasePlayerController_C|GetBaseHUD (Variables|Default|GetPlayerController))))) _returnvalue)
                      (Utilities|Map|Add (Variables|/Game/BluePrints/PlayerController/BP_BasePlayerController.BP_BasePlayerController_C|GetNavPoints (Variables|Default|GetPlayerController)) (Transformation|GetActorLocation) _returnvalue))))))))))))

(fn ConstructionScript)