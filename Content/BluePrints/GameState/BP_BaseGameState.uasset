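; Base game state that tracks free-for-all top scorers and red/blue team scores.
; UpdateTopScore keeps the list of players tied for the highest score, resetting it when someone exceeds it and using AddUnique to avoid duplicates.
; Team score functions increment their totals and push the rounded-up value to player controller 0's HUD.
; RepNotify handlers for both team scores repeat that HUD update when the values replicate.
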(event EventBeginPlay)

(event EventTick
  (params (DeltaSeconds :type Float%20%28single-precision%29)))

(fn ConstructionScript)

(fn UpdateTopScore
  (params (ScoringPlayer :type BP%20Base%20Player%20State%20Object%20Reference))
  (bind _topscoringplayers (Variables|TopScoring|GetTopScoringPlayers))
  ;[1 1 1] If Top Scoring players array is empty -> add the player directly
  (if (== (Utilities|Array|Length (Variables|TopScoring|GetTopScoringPlayers)) 0)
    (Utilities|Array|Add (Variables|TopScoring|GetTopScoringPlayers) ScoringPlayer)
    (Variables|TopScoring|SetTopScore (Variables|/Game/BluePrints/PlayerState/BP_BasePlayerState.BP_BasePlayerState_C|GetPlayerScore ScoringPlayer))
    (else
      ;[1 1 1] If Top score = top score in the array , set it with add unique to avoid replicated element in the array ( multiple winners)
      (if (== (Variables|/Game/BluePrints/PlayerState/BP_BasePlayerState.BP_BasePlayerState_C|GetPlayerScore ScoringPlayer) (Variables|TopScoring|GetTopScore))
        (Utilities|Array|AddUnique (Variables|TopScoring|GetTopScoringPlayers) ScoringPlayer)
        (else
          ;[1 1 1] If the scoring player has a score greater than the top score in the array -> clear the array and add unique score
          (if (> (Variables|/Game/BluePrints/PlayerState/BP_BasePlayerState.BP_BasePlayerState_C|GetPlayerScore ScoringPlayer) (Variables|TopScoring|GetTopScore))
            (Utilities|Array|Clear _topscoringplayers)
            (Utilities|Array|AddUnique _topscoringplayers ScoringPlayer)
            (Variables|TopScoring|SetTopScore (Variables|/Game/BluePrints/PlayerState/BP_BasePlayerState.BP_BasePlayerState_C|GetPlayerScore ScoringPlayer))))))))

(fn OnRepRedTeamScore
  (bind _asbp_base_player_controller (Utilities|Casting|CastToBP_BasePlayerController (Game|GetPlayerController 0)))
  (bind _output_get (LocalVariables|SetBPlayer _asbp_base_player_controller))
  (Utilities|IsValid _output_get
    (:Is%20Valid
      (Default|SetHUDRedTeamScore _output_get (Math|Float|Ceil (Variables|Teams|GetRedTeamScore))))))

(fn RedTeamScores
  (Math|Float|IncrementFloat (Variables|Teams|GetRedTeamScore)
    (:%20%20
      (bind _asbp_base_player_controller (Utilities|Casting|CastToBP_BasePlayerController (Game|GetPlayerController 0)))
      (bind _output_get (LocalVariables|SetBPlayer _asbp_base_player_controller))
      (Utilities|IsValid _output_get
        (:Is%20Valid
          (Default|SetHUDRedTeamScore _output_get (Math|Float|Ceil (Variables|Teams|GetRedTeamScore))))))))

(fn BlueTeamScores
  (Math|Float|IncrementFloat (Variables|Teams|GetBlueTeamScore)
    (:%20%20
      (bind _asbp_base_player_controller (Utilities|Casting|CastToBP_BasePlayerController (Game|GetPlayerController 0)))
      (bind _output_get (LocalVariables|SetBPlayer _asbp_base_player_controller))
      (Utilities|IsValid _output_get
        (:Is%20Valid
          (Default|SetHUDBlueTeamScore _output_get (Math|Float|Ceil (Variables|Teams|GetBlueTeamScore))))))))

(fn OnRepBlueTeamScore
  (bind _asbp_base_player_controller (Utilities|Casting|CastToBP_BasePlayerController (Game|GetPlayerController 0)))
  (bind _output_get (LocalVariables|SetBPlayer _asbp_base_player_controller))
  (Utilities|IsValid _output_get
    (:Is%20Valid
      (Default|SetHUDBlueTeamScore _output_get (Math|Float|Ceil (Variables|Teams|GetBlueTeamScore))))))